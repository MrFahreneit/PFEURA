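; BP_Citizen is a citizen actor shown as a decal, with Peace, Fight and Win looks.
; ChangeCitizenState swaps color and opacity textures on a dynamic material created at BeginPlay, starting in Peace.
; Win starts a self-calling Delay loop that alternates two sprites at a per-instance random interval, with no exit condition.
; The construction script slightly randomizes scale and roll to vary each citizen.
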(event `self.ReceiveBeginPlay`
  (bind _returnvalue (`DecalComponent.CreateDynamicMaterialInstance` (`self.Decal`)))
  (set `self.Mat` _returnvalue)
  (`self.ChangeCitizenState` "NewEnumerator0")
  (set `self.ChangeTime` (`KismetMathLibrary.RandomFloatInRange` 0.2 1.2)))

(event `ChangeCitizenState`
  (params (CurrentState :type "/Game/Interactif/Citizen/Enum_CitizenState Enum" :default "NewEnumerator0"))
  (bind _output_get (set `self.CurrentState` CurrentState))
  (switch `/Game/Interactif/Citizen/Enum_CitizenState` _output_get
    (:`NewEnumerator0`
      (`MaterialInstanceDynamic.SetTextureParameterValue` (`self.Mat`) "BaseColor" (`self.PeaceText`))
      (`MaterialInstanceDynamic.SetTextureParameterValue` (`self.Mat`) "OpacityMap" (`self.PeaceText`)))
    (:`NewEnumerator1`
      (`MaterialInstanceDynamic.SetTextureParameterValue` (`self.Mat`) "BaseColor" (`self.FightTxt`))
      (`MaterialInstanceDynamic.SetTextureParameterValue` (`self.Mat`) "OpacityMap" (`self.FightTxt`)))
    (:`NewEnumerator2`
      (`self.ChangeWinSprite`))))

(event `ChangeWinSprite`
  (bind _isa (`/Engine/EditorBlueprintResources/StandardMacros.FlipFlop`)
    (:`A`
      _)
    (:`B`
      _))
  (`MaterialInstanceDynamic.SetTextureParameterValue` (`self.Mat`) "BaseColor" (select `bool` _isa :`false` (`self.WinTxt1`) :`true` (`self.WinTxt2`)))
  (`MaterialInstanceDynamic.SetTextureParameterValue` (`self.Mat`) "OpacityMap" (select `bool` _isa :`false` (`self.WinTxt1`) :`true` (`self.WinTxt2`)))
  (`KismetSystemLibrary.Delay` (`self.ChangeTime`))
  (`self.ChangeWinSprite`))

(fn `UserConstructionScript`
  (`SceneComponent.SetRelativeScale3D` (`self.ScalePoint`) (`KismetMathLibrary.MakeVector` (`KismetMathLibrary.RandomFloatInRange` 0.9 1.1) (`KismetMathLibrary.RandomFloatInRange` 0.9 1.1) (`KismetMathLibrary.RandomFloatInRange` 0.9 1.1)))
  (`SceneComponent.K2_SetRelativeRotation` (`self.ScalePoint`) (`KismetMathLibrary.MakeRotator` (`KismetMathLibrary.RandomFloatInRange` -3.0 3.0)) false false))