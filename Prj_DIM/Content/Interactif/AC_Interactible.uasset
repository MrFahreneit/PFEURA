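; Actor component that gives an interactible a prompt widget and can move the player into position on interaction.
; Init spawns a widget actor attached to a given point, hidden by default; Show reveals it only while the component is active.
; If movement is enabled, ActivateMovement disables player input and starts a timer, during which Tick interpolates the player toward a target transform.
; When the timer ends, input is optionally restored.
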(event `ActivateMovement`
  (if (`self.InteractMovement`)
    (`KismetSystemLibrary.K2_ClearAndInvalidateTimerHandle` (`self.TimerMovement`))
    (bind _returnvalue (`KismetSystemLibrary.K2_SetTimerDelegate` (delegate `StopMovementTime`) (`self.timeMovement`)))
    (set `self.TimerMovement` _returnvalue)
    (bind _output_get (set `self.ActionActor` (`GameplayStatics.GetPlayerCharacter` 0)))
    (`Actor.DisableInput` _output_get (`GameplayStatics.GetPlayerController` 0))))

(event `Init`
  (params (Point :type "SceneComponent Object Reference"))
  (bind _returnvalue (`|SpawnActorFromClass` "/Game/Interactif/BP_InteractibleWidget.BP_InteractibleWidget_C" (`KismetMathLibrary.MakeTransform` (0.0 0.0 0.0)) "AlwaysSpawn" "OverrideRootScale" null null))
  (set `self.BP_Widget` _returnvalue)
  (`Actor.K2_AttachToComponent` _returnvalue Point "None" "KeepRelative" "KeepRelative" "KeepRelative" true)
  (`SceneComponent.SetHiddenInGame` (`/Game/Interactif/BP_InteractibleWidget.Widget` _returnvalue) true true))

(event `StopMovementTime`
  (`KismetSystemLibrary.K2_ClearAndInvalidateTimerHandle` (`self.TimerMovement`))
  (if (`self.ReEnableInputAfter`)
    (`Actor.EnableInput` (`self.ActionActor`) (`GameplayStatics.GetPlayerController` 0))))

(event `self.ReceiveTick`
  (params (DeltaSeconds :type "Float (single-precision)"))
  (bind _movementforce (`self.movementForce`))
  (bind _actionactor (`self.ActionActor`))
  (bind (_returnvalue_location _returnvalue_rotation) (`KismetMathLibrary.BreakTransform` (`SceneComponent.K2_GetComponentToWorld` (`self.ObjectifMovement`))))
  (bind (_returnvalue_location_2 _returnvalue_rotation_2) (`KismetMathLibrary.BreakTransform` (`Actor.GetTransform` _actionactor)))
  (if (`KismetSystemLibrary.K2_IsValidTimerHandle` (`self.TimerMovement`))
    (`/Engine/EditorBlueprintResources/StandardMacros.IsValid` _actionactor
      (:`Is Valid`
        (`Actor.K2_SetActorTransform` _actionactor (`KismetMathLibrary.MakeTransform` (`KismetMathLibrary.VInterpTo` _returnvalue_location_2 _returnvalue_location DeltaSeconds _movementforce) (`KismetMathLibrary.RInterpTo` _returnvalue_rotation_2 _returnvalue_rotation DeltaSeconds _movementforce)) false true)))))

(event `Show`
  (params (`On?` :type Boolean))
  (bind _widget (`/Game/Interactif/BP_InteractibleWidget.Widget` (`self.BP_Widget`)))
  (if `On?`
    (if (`self.isActive?`)
      (`SceneComponent.SetHiddenInGame` _widget false true)
      (else
        (`SceneComponent.SetHiddenInGame` _widget true true :!label _label)))
    (else
      (goto _label))))

(event `ChangeState`
  (params (`isActive?` :type Boolean))
  (set `self.isActive?` `isActive?`))