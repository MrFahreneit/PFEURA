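; BP_Projectile is a stationary enemy laser attack that locks onto the player and can be evaded by dashing.
; On BeginPlay it spawns a targeting Niagara beam, then after a fixed delay fires the main beam and damages the player if still tracking, without a collision test.
; Tick keeps both beam ends on the player until HasDashed sets StopFollow, after which the fired beam extends past the last tracked position.
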(event `self.ReceiveBeginPlay`
  (bind _asbp_player (cast `/Game/Player/BP_Player` (`GameplayStatics.GetPlayerCharacter` 0)))
  (bind _output_get (set `self.As BP Player` _asbp_player))
  (add `/Game/Player/BP_Player.HasDashed` _output_get (delegate `StopFollowing`))
  (`self.SpawnParticle`)
  (`KismetSystemLibrary.K2_SetTimer` null "SpawnParticle" 4.0 true)
  (bind _returnvalue (`NiagaraFunctionLibrary.SpawnSystemAttached` "/Game/GA/NiagaraSystems/NS_ProjectileEnemyLaserCible.NS_ProjectileEnemyLaserCible" (`self.Scene`) "None" (`self.K2_GetActorLocation`) (struct) "KeepWorldPosition"))
  (bind _output_get_2 (set `self.laserSpawned` _returnvalue))
  (`FXSystemComponent.SetVectorParameter` _output_get_2 "BeamEnd" (`self.K2_GetActorLocation` (`GameplayStatics.GetPlayerCharacter` 0)))
  (`KismetSystemLibrary.Delay` 2.7)
  (bind _returnvalue_2 (`NiagaraFunctionLibrary.SpawnSystemAttached` "/Game/GA/NiagaraSystems/NS_ProjectileEnemyLaserEM.NS_ProjectileEnemyLaserEM" (`self.Scene`) "None" (`self.K2_GetActorLocation`) (struct) "KeepWorldPosition"))
  (set `self.Cible` _returnvalue_2)
  (`FXSystemComponent.SetVectorParameter` _returnvalue_2 "BeamEnd" (select `bool` (`self.stopFollow`) :`false` (`self.BeamEnd`) :`true` (+ (`self.K2_GetActorLocation`) (* (`KismetMathLibrary.Normal` (- (`self.BeamEnd`) (`self.K2_GetActorLocation`))) 10000.0))))
  (if (not (`self.stopFollow`))
    (`/Game/Player/BP_Player.LoseHealth` (`self.As BP Player`) (`self.Damages`))))

(event `StopFollowing`
  (set `self.stopFollow` true))

(event `SpawnParticle`)

(event `self.ReceiveTick`
  (params (DeltaSeconds :type "Float (single-precision)"))
  (bind _cible (`self.Cible`))
  (bind _laserspawned (`self.laserSpawned`))
  (bind _beamend (`self.BeamEnd`))
  (if (not (`self.stopFollow`))
    (set `self.BeamEnd` (`self.K2_GetActorLocation` (`GameplayStatics.GetPlayerCharacter` 0)))
    (`/Engine/EditorBlueprintResources/StandardMacros.IsValid` _cible
      (:`Is Valid`
        (`FXSystemComponent.SetVectorParameter` _cible "BeamEnd" _beamend))
      (:`Is Not Valid`
        _))
    (`/Engine/EditorBlueprintResources/StandardMacros.IsValid` _laserspawned
      (:`Is Valid`
        (`FXSystemComponent.SetVectorParameter` _laserspawned "BeamEnd" (select `bool` (`self.stopFollow`) :`false` _beamend :`true` (+ (`self.K2_GetActorLocation`) (* (`KismetMathLibrary.Normal` (- (`self.BeamEnd`) (`self.K2_GetActorLocation`))) 10000.0))))))))

(fn `UserConstructionScript`)