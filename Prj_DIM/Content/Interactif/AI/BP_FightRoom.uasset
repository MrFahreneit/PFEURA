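; Arena actor that runs a combat encounter, started when the player first overlaps its box, with optional boss-room support.
; On start it raises walls, switches citizens and 1D lines, and spawns enemies up to the wave budget through ACWaveManager.
; It tracks spawned enemies, relays attack notifications, pauses them for combo finishers and repositions them for boss phases.
; When the tracked list empties, it destroys the walls and ends the fight.
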(event `TeleportBossPhase2Here`
  (for _array_element (`self.EnemySpawned`)
    (`self.K2_SetActorLocation` _array_element (`self.K2_GetActorLocation` (`self.TeleportBossPhase2`)) false true)))

(event `Eject1DAnimBoss`
  (bind _pointzoneeject1 (`self.pointZoneEject1`))
  (for _array_element (`self.EnemySpawned`)
    (bind _output_get (set `/Game/Interactif/AI/AI_Master.PointMovementForce` (`self.K2_GetActorLocation` _pointzoneeject1) _array_element))
    (`self.K2_SetActorLocation` _array_element _output_get false true)
    (`self.K2_SetActorRotation` _array_element (`self.K2_GetActorRotation` _pointzoneeject1) false)
    (`/Game/Interactif/AI/AI_Master.StartEject1D` _array_element)))

(event `NextPhaseBoss`
  (bind _phase2bossmover (`self.Phase2BossMover`))
  (`/Game/Interactif/TriggerBox/BP_PlayeraBossMover.Spawn1DPoint` _phase2bossmover)
  (for _array_element (`self.EnemySpawned`)
    (set `/Game/Interactif/AI/AI_Master.PointMovementForce` (`self.K2_GetActorLocation` (`/Game/Interactif/TriggerBox/BP_PlayeraBossMover.PointEntering1D` _phase2bossmover)) _array_element)
    (`/Game/Interactif/AI/AI_Master.ChangeAIBehavior` _array_element "NewEnumerator9" true)))

(event `self.ReceiveBeginPlay`
  (bind _phase2bossmover (`self.Phase2BossMover`))
  (`/Game/Interactif/AI/WaveSystem/AC_WaveManager.InitializeWaveManager` (`self.AC_WaveManager`) (`self.Waves`) (`self.WaveSpawnPoints`))
  (add `/Game/Interactif/AI/WaveSystem/AC_WaveManager.EntitySpawned` (`self.AC_WaveManager`) (`|CreateDelegate` :!event `OnEntitySpawned`))
  (add `/Game/Interactif/AI/WaveSystem/AC_WaveManager.LastEntitySpawned` (`self.AC_WaveManager`) (`|CreateDelegate` :!event `OnLastEntitySpawned`))
  (for _array_element (`self.FightWalls`)
    (`self.SetActorHiddenInGame` _array_element true)
    (`self.SetActorEnableCollision` _array_element false))
  (if (`self.bossRoom`)
    (`/Engine/EditorBlueprintResources/StandardMacros.IsValid` _phase2bossmover
      (:`Is Valid`
        (set `/Game/Interactif/TriggerBox/BP_PlayeraBossMover.FightRoom` self _phase2bossmover)))))

(event `self.Box.OnComponentBeginOverlap`
  (params (OverlappedComponent :type "PrimitiveComponent Object Reference") (OtherActor :type "Actor Object Reference") (OtherComp :type "PrimitiveComponent Object Reference") (OtherBodyIndex :type Integer) (bFromSweep :type Boolean) (SweepResult :type "HitResult Structure (by ref)"))
  (bind _asbp_player (cast `/Game/Player/BP_Player` OtherActor))
  (`/Engine/EditorBlueprintResources/StandardMacros.DoOnce` false
    (:`Completed`
      (set `self.BP_Player` _asbp_player)
      (set `/Game/Player/BP_Player.currentFightRoom` self _asbp_player)
      (`self.StartFight`))))

(event `OnEntitySpawned`
  (params (Entity :type "Actor Object Reference"))
  (bind _asai_master (cast `/Game/Interactif/AI/AI_Master` Entity))
  (if (`/Game/Interactif/AI/AI_Master.isBoss?` _asai_master)
    (set `/Game/Interactif/AI/AI_Master.BP_FightRoom` self _asai_master)
    (else
      (`/Game/Interactif/AI/AI_Master.InitEnemy` _asai_master self)))
  (`KismetArrayLibrary.Array_AddUnique` (`self.EnemySpawned`) _asai_master)
  (add `/Game/Interactif/AI/AI_Master.AttackingEvent` _asai_master (`|CreateDelegate` :!event `SomeoneHasAttack`))
  (add `/Game/Interactif/AI/AC_HealthComponent.HasBeenKilled` (`/Game/Interactif/AI/AI_Master.AC_HealthComponent` _asai_master) (`|CreateDelegate` :!event `OnHasBeenKilled`)))

(event `StartFight`
  (bind _ejectteleport (`self.EjectTeleport`))
  (bind _hud_widget (`/Game/Player/BP_Player.HUD_Widget` (`self.BP_Player`)))
  (bind _asbp_player (cast `/Game/Player/BP_Player` (`GameplayStatics.GetPlayerCharacter` 0)))
  (bind _output_get (set `self.BP_Player` _asbp_player))
  (set `/Game/Player/BP_Player.currentFightRoom` self _output_get)
  (`/Engine/EditorBlueprintResources/StandardMacros.IsValid` _ejectteleport
    (:`Is Valid`
      (set `/Game/Interactif/1DTravel/BP_1DTeleport.fightRoom` self _ejectteleport))
    (:`Is Not Valid`
      _))
  (set `/Game/Player/BP_Player.IsInFight` true (`self.BP_Player`))
  (set `self.isOn?` true)
  (if (not (`self.bossRoom`))
    (`UserWidget.PlayAnimation` _hud_widget (`/Game/UI/Widgets/HUD/W_HUD.ShowInputs` _hud_widget) 0.0 1 "Forward" 1.0 false))
  (for _array_element (`self.Citizens`)
    (`/Engine/EditorBlueprintResources/StandardMacros.IsValid` _array_element
      (:`Is Valid`
        (`/Game/Interactif/Citizen/BP_Citizen.ChangeCitizenState` _array_element "NewEnumerator1"))))
  (for _array_element_2 (`self.1DLines`)
    (`/Engine/EditorBlueprintResources/StandardMacros.IsValid` _array_element_2
      (:`Is Valid`
        (`/Game/Interactif/1DTravel/BP_1DSpline.ChangeState` _array_element_2 true))))
  (for _array_element_3 (`self.FightWalls`)
    (`self.SetActorHiddenInGame` _array_element_3 false)
    (`self.SetActorEnableCollision` _array_element_3 true))
  (for _ (range 1 (+ (`.Budget_2_70006EC14A2837ED8F3E87A54B31AC5C` (break `/Game/Interactif/AI/WaveSystem/S_Wave` (`/Game/Interactif/AI/WaveSystem/AC_WaveManager.GetCurrentWave` (`self.AC_WaveManager`)))) 1))
    (bind _spawnsuccess (`/Game/Interactif/AI/WaveSystem/AC_WaveManager.TrySpawnEntity` (`self.AC_WaveManager`)))
    (if (not _spawnsuccess)
      (break))))

(event `SomeoneHasAttack`
  (params (`Start?` :type Boolean) (`Who?` :type "/Game/Interactif/AI/AI_Master Object Reference"))
  (set `self.LastAttacker` `Who?`)
  (set `self.someoneAttack` `Start?`)
  (for _array_element (`self.EnemySpawned`)
    (`/Engine/EditorBlueprintResources/StandardMacros.IsValid` _array_element
      (:`Is Valid`
        (if `Start?`
          (`/Game/Interactif/AI/AI_Master.SomeoneIsAttacking` _array_element `Who?`)
          (else
            (`/Game/Interactif/AI/AI_Master.OtherIsAttackingStop` _array_element)))))))

(event `BindWaveEvents`
  ;[0.3698 0.3698 0.3698] OBSOLETE SYSTEM
  (for _array_element (`self.EnemySpawned`)
    (bind _returnvalue (`self.GetComponentByClass` _array_element "/Game/Interactif/AI/AC_HealthComponent.AC_HealthComponent_C"))
    (if (`KismetSystemLibrary.IsValid` _returnvalue)
      (`/Game/Interactif/AI/WaveSystem/AC_WaveManager.BindOnKilledEvent` (`self.AC_WaveManager`) _returnvalue))))

(event `FightFinished`
  (bind _hud_widget (`/Game/Player/BP_Player.HUD_Widget` (`self.BP_Player`)))
  (`KismetSystemLibrary.PrintString` "FIGHT FINISHED" true false (struct :`G` 1.0 :`B` 0.051528 :`A` 1.0) 10.0)
  (set `self.isOn?` false)
  (set `/Game/Player/BP_Player.IsInFight` false (`self.BP_Player`))
  (`UserWidget.PlayAnimation` _hud_widget (`/Game/UI/Widgets/HUD/W_HUD.ShowInputs` _hud_widget) 0.0 1 "Reverse" 1.0 false)
  (`self.FinishedFight`)
  (for _array_element (`self.FightWalls`)
    (`self.K2_DestroyActor` _array_element))
  (for _array_element_2 (`self.Citizens`)
    (`/Engine/EditorBlueprintResources/StandardMacros.IsValid` _array_element_2
      (:`Is Valid`
        (`/Game/Interactif/Citizen/BP_Citizen.ChangeCitizenState` _array_element_2 "NewEnumerator2"))))
  (for _array_element_3 (`self.1DLines`)
    (`/Engine/EditorBlueprintResources/StandardMacros.IsValid` _array_element_3
      (:`Is Valid`
        (`/Game/Interactif/1DTravel/BP_1DSpline.ChangeState` _array_element_3 false)))))

(event `PauseAllOther`
  (params (`Who Instigate` :type "/Game/Interactif/AI/AI_Master Object Reference"))
  (for _array_element (`self.EnemySpawned`)
    (`/Engine/EditorBlueprintResources/StandardMacros.IsValid` _array_element
      (:`Is Valid`
        (if (!= _array_element `Who Instigate`)
          (`/Game/Interactif/AI/AC_ComboFinisherPauser.PauseActor` (`/Game/Interactif/AI/AI_Master.AC_ComboFinisherPauser` _array_element)))))))

(event `UnpauseAllActor`
  (for _array_element (`self.EnemySpawned`)
    (`/Engine/EditorBlueprintResources/StandardMacros.IsValid` _array_element
      (:`Is Valid`
        (`/Game/Interactif/AI/AC_ComboFinisherPauser.UnpauseActor` (`/Game/Interactif/AI/AI_Master.AC_ComboFinisherPauser` _array_element))))))

(fn `OnHasBeenKilled`
  (params (KilledActor :type "Actor Object Reference"))
  (bind _asai_master (cast `/Game/Interactif/AI/AI_Master` KilledActor))
  (`KismetArrayLibrary.Array_RemoveItem` (`self.EnemySpawned`) _asai_master)
  (if (`KismetArrayLibrary.Array_IsEmpty` (`self.EnemySpawned`))
    (`self.FightFinished`)))

(fn `OnLastEntitySpawned`
  (set `self.LastEntitySpawned` true))

(fn `UserConstructionScript`)