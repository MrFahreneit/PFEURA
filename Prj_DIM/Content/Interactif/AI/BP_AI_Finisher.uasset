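; BP_AI_Finisher is a one-shot interactible owned by an AI_Master, apparently a finisher prompt on that AI.
; BeginPlay initializes ACInteractible with the interactor widget, sets TargetPoint as its movement objective and caches the owning AI.
; Interaction disables and hides the interactible, sends a start-interact message to the AI, activates movement, then destroys the actor after a short delay.
; ShowInteractIcon toggles the prompt's visibility.
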(event `/Game/Interactif/BPI_Interactible.START_INTERACTION`
  (bind _ac_interactible (`self.AC_Interactible`))
  (`/Engine/EditorBlueprintResources/StandardMacros.DoOnce` false
    (:`Completed`
      (`/Game/Interactif/AC_Interactible.ChangeState` _ac_interactible false)
      (`/Game/Interactif/AC_Interactible.Show` _ac_interactible false)
      (message `/Game/Interactif/BPI_ActorInteract.StartEventInteract` (`self.OwnerBP`) 0)
      (`/Game/Interactif/AC_Interactible.ActivateMovement` (`self.AC_Interactible`))
      (`KismetSystemLibrary.Delay` 2.0)
      (`self.K2_DestroyActor`))))

(event `/Game/Interactif/BPI_Interactible.ShowInteractIcon`
  (params (`On?` :type Boolean))
  ;[1 1 1] ToCopy
  (`/Game/Interactif/AC_Interactible.Show` (`self.AC_Interactible`) `On?`))

(event `self.ReceiveBeginPlay`
  (bind _ac_interactible (`self.AC_Interactible`))
  ;[1 1 1] ToCopy
  (`/Game/Interactif/AC_Interactible.Init` (`self.AC_Interactible`) (`self.InteractorWidget`))
  (`/Game/Interactif/AC_Interactible.Init` _ac_interactible (`self.InteractorWidget`))
  (set `/Game/Interactif/AC_Interactible.ObjectifMovement` (`self.TargetPoint`) _ac_interactible)
  (bind _asai_master (cast `/Game/Interactif/AI/AI_Master` (`self.GetOwner`)))
  (set `self.OwnerBP` _asai_master))

(fn `UserConstructionScript`)