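; Wave manager component that spawns enemies under a per-wave cost budget, cycling through each wave's entity list.
; Melee enemies use random spawn points without repeats until all are used; ranged enemies target the point furthest from the player.
; Health component death events refund budget and trigger replacement spawns.
; Kill thresholds advance non-endless waves, refilling the new budget, until the last wave stops spawning and signals completion.
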(event `BindOnKilledEvent`
  (params (HealthComponent :type "/Game/Interactif/AI/AC_HealthComponent Object Reference"))
  (add `/Game/Interactif/AI/AC_HealthComponent.HasBeenKilled` HealthComponent (`|CreateDelegate` :!event `OnKilled`)))

(fn `GetCurrentEntity`
  (returns (CurrentEntityToSpawn :type "/Game/Interactif/AI/WaveSystem/S_WaveEntity Structure"))
  (return (`|GetArrayItem` (`.EntitiesToSpawn_15_43B13B29423ED2636B38B78360A8550B` (break `/Game/Interactif/AI/WaveSystem/S_Wave` (`self.GetCurrentWave`))) (`self.EntityIndex`))))

(fn `GetCurrentWave`
  (returns (CurrentWave :type "/Game/Interactif/AI/WaveSystem/S_Wave Structure (by ref)"))
  (return (`|GetArrayItem` (`self.Waves`) (`self.WaveIndex`))))

(fn `GetSpawner`
  (returns (SelectedSpawner :type "/Game/Interactif/AI/WaveSystem/BP_WaveSpawnPoint Object Reference"))
  (locals (SelectedBis :type "/Game/Interactif/AI/WaveSystem/BP_WaveSpawnPoint Object Reference") (FurthestDistance :type "Float (double-precision)") (TestedMeleeIndex :type Integer))
  (switch `/Game/Interactif/AI/WaveSystem/E_EntityType` (`.EntityType_12_5D28B37F432E2381A629E1BFF781FE96` (break `/Game/Interactif/AI/WaveSystem/S_WaveEntity` (`self.GetCurrentEntity`)))
    (:`NewEnumerator1`
      ;[1 1 1] Get Melee Spawn Point
      (set `local.TestedMeleeIndex` (`KismetMathLibrary.RandomInteger` (`KismetArrayLibrary.Array_Length` (`self.MeleeSpawner`))) :!label _label)
      (if (not (`KismetArrayLibrary.Array_Contains` (`self.MeleeUsedIndex`) (`local.TestedMeleeIndex`)))
        (set `local.SelectedBis` (`|GetArrayItem` (`self.MeleeSpawner`) (`local.TestedMeleeIndex`)))
        (`KismetArrayLibrary.Array_AddUnique` (`self.MeleeUsedIndex`) (`local.TestedMeleeIndex`))
        (if (>= (`KismetArrayLibrary.Array_Length` (`self.MeleeUsedIndex`)) (`KismetArrayLibrary.Array_Length` (`self.MeleeSpawner`)))
          (`KismetArrayLibrary.Array_Clear` (`self.MeleeUsedIndex`)))
        (return (`local.SelectedBis`))
        (else
          (goto _label))))
    (:`NewEnumerator2`
      ;[1 1 1] Get Ranged Spawn Point
      (for _array_element (`self.WaveSpawnPoints`)
        (if (`|EnumEquality` (`/Game/Interactif/AI/WaveSystem/BP_WaveSpawnPoint.SpawnerType` _array_element) "NewEnumerator2")
          (bind _returnvalue (`KismetMathLibrary.Vector_DistanceSquared` (`Actor.K2_GetActorLocation` _array_element) (`Actor.K2_GetActorLocation` (`GameplayStatics.GetPlayerCharacter` 0))))
          (if (> _returnvalue (`local.FurthestDistance`))
            (set `local.FurthestDistance` _returnvalue)
            (set `local.SelectedBis` _array_element))))
      (return (`local.SelectedBis`)))))

(fn `IncrementEntityIndex`
  (bind _returnvalue (+ (`self.EntityIndex`) 1))
  (if (> _returnvalue (`KismetArrayLibrary.Array_LastIndex` (`.EntitiesToSpawn_15_43B13B29423ED2636B38B78360A8550B` (break `/Game/Interactif/AI/WaveSystem/S_Wave` (`self.GetCurrentWave`)))))
    (set `self.EntityIndex` 0)
    (else
      (set `self.EntityIndex` _returnvalue))))

(fn `IncrementWaveIndex`
  (`KismetSystemLibrary.PrintString` "NEXT WAVE" true false (struct :`R` 1.0 :`G` 0.565984 :`A` 1.0) 5.0)
  (if (> (+ (`self.WaveIndex`) 1) (`KismetArrayLibrary.Array_LastIndex` (`self.Waves`)))
    (`self.LastEntitySpawned`)
    (set `self.IsDoneSpawning` true)
    (`KismetSystemLibrary.PrintString` "LAST WAVE" true false (struct :`R` 1.0 :`G` 0.446525 :`A` 1.0) 5.0)
    (else
      (`/Engine/EditorBlueprintResources/StandardMacros.IncrementInt` (`self.WaveIndex`)
        (:`  `
          (set `self.CurrentKilledCount` 0)
          (set `self.EntityIndex` 0)
          (for _ (range 1 (+ (`.Budget_2_70006EC14A2837ED8F3E87A54B31AC5C` (break `/Game/Interactif/AI/WaveSystem/S_Wave` (`self.GetCurrentWave`))) 1))
            (bind _spawnsuccess (`self.TrySpawnEntity`))
            (if (not _spawnsuccess)
              (break))))))))

(fn `InitializeWaveManager`
  (params (Waves :type "Array of /Game/Interactif/AI/WaveSystem/S_Wave Structure") (WaveSpawnPoints :type "Array of /Game/Interactif/AI/WaveSystem/BP_WaveSpawnPoint Object Reference"))
  (set `self.Waves` Waves)
  (bind _output_get (set `self.WaveSpawnPoints` WaveSpawnPoints))
  (for _array_element _output_get
    (if (`|EnumEquality` (`/Game/Interactif/AI/WaveSystem/BP_WaveSpawnPoint.SpawnerType` _array_element) "NewEnumerator1")
      (`KismetArrayLibrary.Array_AddUnique` (`self.MeleeSpawner`) _array_element))))

(fn `OnKilled`
  (params (KilledActor :type "Actor Object Reference"))
  (bind _returnvalue (`Actor.GetComponentByClass` KilledActor "/Game/Interactif/AI/WaveSystem/AC_WaveEntity.AC_WaveEntity_C"))
  (bind _currentkilledcount (`self.CurrentKilledCount`))
  (bind (_isendless _budget _killtonextbudget) (break `/Game/Interactif/AI/WaveSystem/S_Wave` (`self.GetCurrentWave`)))
  (if (`KismetSystemLibrary.IsValid` _returnvalue)
    (set `self.CurrentBudgetCost` (- (`self.CurrentBudgetCost`) (`/Game/Interactif/AI/WaveSystem/AC_WaveEntity.BudgetCost` _returnvalue)))
    (`/Engine/EditorBlueprintResources/StandardMacros.IncrementInt` _currentkilledcount
      (:`  `
        (if (>= _currentkilledcount _killtonextbudget)
          (if _isendless
            (if (not (`self.IsDoneSpawning`)) :!label _label
              (`self.TrySpawnEntity`))
            (elif (not (`self.IsDoneSpawning`))
              (`self.IncrementWaveIndex`)
              (goto _label)))
          (else
            (goto _label)))))
    (else
      (`KismetSystemLibrary.PrintString` "KILLED ACTOR DOES NOT HAVE AC_WAVE_ENTITY" true false (struct :`R` 1.0 :`G` 0.026767 :`A` 1.0) 20.0))))

(fn `TrySpawnEntity`
  (returns (SpawnSuccess :type Boolean))
  (bind (_entitytospawn _entitytype _budgetcost) (break `/Game/Interactif/AI/WaveSystem/S_WaveEntity` (`self.GetCurrentEntity`)))
  (if (not (> (+ (`.BudgetCost_11_BC3209F74FA299304B8058A649C99A0C` (break `/Game/Interactif/AI/WaveSystem/S_WaveEntity` (`self.GetCurrentEntity`))) (`self.CurrentBudgetCost`)) (`.Budget_2_70006EC14A2837ED8F3E87A54B31AC5C` (break `/Game/Interactif/AI/WaveSystem/S_Wave` (`self.GetCurrentWave`)))))
    (bind _returnvalue (`|SpawnActorFromClass` _entitytospawn (`Actor.GetTransform` (`self.GetSpawner`)) "AdjustIfPossibleButAlwaysSpawn" "OverrideRootScale" null null)) ; Always Spawn or else get Pending Kill / Garbage Error
    (`self.IncrementEntityIndex`)
    (bind _returnvalue_2 (`Actor.GetComponentByClass` _returnvalue "/Game/Interactif/AI/AC_HealthComponent.AC_HealthComponent_C"))
    (if (`KismetSystemLibrary.IsValid` _returnvalue_2)
      (`self.BindOnKilledEvent` _returnvalue_2)
      (set `self.CurrentBudgetCost` (+ (`self.CurrentBudgetCost`) _budgetcost))
      (`self.EntitySpawned` _returnvalue)
      (return true)
      (else
        (`KismetSystemLibrary.PrintString` "SPAWNED ACTOR DOES NOT HAVE AC_HEALTHCOMPONENT" true false (struct :`R` 1.0 :`G` 0.026767 :`A` 1.0) 20.0)
        (return true)))
    (else
      (return false))))