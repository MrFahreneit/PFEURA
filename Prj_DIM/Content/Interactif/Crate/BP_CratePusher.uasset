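; BP_CratePusher is an interactible push point that lets the player shove crates or other linked actors.
; An ACInteractible component handles the interact icon and active state, with PushPoint set as its movement objective on BeginPlay.
; When interaction starts while active, it calls PlayrPushBlock on the player, waits briefly, then sends StartEventInteractMessage with its Side to every actor in ActorToInteract.
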(event `/Game/Interactif/BPI_Interactible.START_INTERACTION`
  (if (`/Game/Interactif/AC_Interactible.isActive?` (`self.AC_Interactible`))
    (bind _asbp_player (cast `/Game/Player/BP_Player` (`GameplayStatics.GetPlayerCharacter` 0)))
    (`/Game/Player/BP_Player.PlayrPushBlock` _asbp_player)
    (`KismetSystemLibrary.Delay` 0.45)
    (for _array_element (`self.ActorToInteract`)
      (message `/Game/Interactif/BPI_ActorInteract.StartEventInteract` _array_element (`self.Side?`)))))

(event `/Game/Interactif/BPI_Interactible.ShowInteractIcon`
  (params (`On?` :type Boolean))
  ;[1 1 1] ToCopy
  (`/Game/Interactif/AC_Interactible.Show` (`self.AC_Interactible`) `On?` false))

(event `self.ReceiveBeginPlay`
  (bind _ac_interactible (`self.AC_Interactible`))
  ;[1 1 1] ToCopy
  (`/Game/Interactif/AC_Interactible.Init` _ac_interactible (`self.InteractorWidget`))
  (set `/Game/Interactif/AC_Interactible.ObjectifMovement` (`self.PushPoint`) _ac_interactible))

(fn `UserConstructionScript`)