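; BP_TutoTrigger is a trigger volume that shows a tutorial on the player's HUD the first time a player enters it.
; On box overlap it gets the HUD widget from BP_Player, or through the linked BP_Player reference when the actor is a BP_2DPlayer.
; Both paths share a DoOnce, so MakeTutorial is called with the Tutorial variable only once.
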(event `self.Box.OnComponentBeginOverlap`
  (params (OverlappedComponent :type "PrimitiveComponent Object Reference") (OtherActor :type "Actor Object Reference") (OtherComp :type "PrimitiveComponent Object Reference") (OtherBodyIndex :type Integer) (bFromSweep :type Boolean) (SweepResult :type "HitResult Structure (by ref)"))
  (bind _asbp_player (cast `/Game/Player/BP_Player` OtherActor)
    (:`then`
      (set `self.HUDWidget` (`/Game/Player/BP_Player.HUD_Widget` _asbp_player)))
    (:`CastFailed`
      (bind _asbp_2dplayer (cast `/Game/Player/2DPlayer/BP_2DPlayer` OtherActor))
      (set `self.HUDWidget` (`/Game/Player/BP_Player.HUD_Widget` (`/Game/Player/2DPlayer/BP_2DPlayer.As BP Player` _asbp_2dplayer)))))
  (`/Engine/EditorBlueprintResources/StandardMacros.DoOnce` false
    (:`Completed`
      (`/Game/UI/Widgets/HUD/W_HUD.MakeTutorial` (`self.HUDWidget`) (`self.Tutorial`)))))

(fn `UserConstructionScript`)