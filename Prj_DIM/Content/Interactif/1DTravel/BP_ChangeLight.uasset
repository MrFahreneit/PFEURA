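; BP_ChangeLight is a Blueprint that switches the level's lighting or look by toggling two lists of actors, ENABLES and DISABLES.
; Its ChangeLight event sets post-process volumes in ENABLES to unbound and unhides the other actors, then does the reverse for DISABLES.
; Invalid entries are skipped, and a debug "Hello" prints once both lists are processed.
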(event `ChangeLight`
  (for _array_element (`self.ENABLES`)
    (`/Engine/EditorBlueprintResources/StandardMacros.IsValid` _array_element
      (:`Is Valid`
        (bind _aspost_process_volume (cast `PostProcessVolume` _array_element)
          (:`then`
            (set `PostProcessVolume.bUnbound` true _aspost_process_volume))
          (:`CastFailed`
            (`self.SetActorHiddenInGame` _array_element false))))))
  (for _array_element_2 (`self.DISABLES`)
    (`/Engine/EditorBlueprintResources/StandardMacros.IsValid` _array_element_2
      (:`Is Valid`
        (bind _aspost_process_volume_2 (cast `PostProcessVolume` _array_element_2)
          (:`then`
            (set `PostProcessVolume.bUnbound` false _aspost_process_volume_2))
          (:`CastFailed`
            (`self.SetActorHiddenInGame` _array_element_2 true))))))
  (`KismetSystemLibrary.PrintString` "Hello"))

(fn `UserConstructionScript`)