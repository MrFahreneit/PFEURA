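; BP_1DController is a pawn for one-dimensional travel, moved along the world Y axis by player input.
; The Enhanced Input action IA_Move feeds its X value into the Y component of the movement direction.
; A disconnected chain would disable the player character's input, possess this pawn and add IMC_Default, but it never runs, so the file itself does not take control.
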(event `self.ReceiveBeginPlay`)

(event `EnhancedInput|/Game/ThirdPerson/Input/Actions/IA_Move`
  (params (ActionValue :type "Vector2D Structure") (ElapsedSeconds :type "Float (double-precision)") (TriggeredSeconds :type "Float (double-precision)") (InputAction :type "InputAction Object Reference" :default "/Game/ThirdPerson/Input/Actions/IA_Move.IA_Move"))
  (:`Triggered`
    (`self.AddMovementInput` (`KismetMathLibrary.MakeVector` 0.0 ActionValue_X))))

(fn `UserConstructionScript`)