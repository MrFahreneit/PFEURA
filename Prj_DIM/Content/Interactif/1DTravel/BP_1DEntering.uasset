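; BP_1DEntering is a one-shot interactable that moves the player into the game's 1D travel mode.
; Its ACInteractible component handles the interact icon and activates the objective movement when interaction starts.
; Interaction calls PlayerEnter1D on BP_Player, blends the view to this actor, then after a delay messages every actor in ActorToInteract.
; If MoveAfterInteract is set, it then teleports itself far below the level.
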(event `/Game/Interactif/BPI_Interactible.START_INTERACTION`
  (`/Engine/EditorBlueprintResources/StandardMacros.DoOnce` false
    (:`Completed`
      (`/Game/Interactif/AC_Interactible.ActivateMovement` (`self.AC_Interactible`))
      (bind _asbp_player (cast `/Game/Player/BP_Player` (`GameplayStatics.GetPlayerCharacter` 0)))
      (`/Game/Player/BP_Player.Player Enter 1D` _asbp_player)
      (`PlayerController.SetViewTargetWithBlend` (`GameplayStatics.GetPlayerController` 0) self 1.0 "VTBlend_Cubic" 1.0 false)
      (`KismetSystemLibrary.Delay` 1.5)
      (for _array_element (`self.ActorToInteract`)
        (message `/Game/Interactif/BPI_ActorInteract.StartEventInteract` _array_element 0))
      (if (`self.MoveAfterInteract?`)
        (`KismetSystemLibrary.Delay` 1.0)
        (`self.K2_SetActorLocation` (0.0 0.0 -10000.0))))))

(event `/Game/Interactif/BPI_Interactible.ShowInteractIcon`
  (params (`On?` :type Boolean))
  ;[1 1 1] ToCopy
  (`/Game/Interactif/AC_Interactible.Show` (`self.AC_Interactible`) `On?`))

(event `self.ReceiveBeginPlay`
  (bind _ac_interactible (`self.AC_Interactible`))
  ;[1 1 1] ToCopy
  (`/Game/Interactif/AC_Interactible.Init` _ac_interactible (`self.InteractorWidget`))
  (set `/Game/Interactif/AC_Interactible.ObjectifMovement` (`self.MovementObj`) _ac_interactible))

(fn `UserConstructionScript`)