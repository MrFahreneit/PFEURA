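; BP_1DPassenger is a passenger marker that travels once along a 1DLine spline and then destroys itself.
; On BeginPlay it gives its plane a dynamic masked unlit material with a random color from a fixed palette.
; A timeline, rate-scaled by spline length over Speed for constant velocity, moves the actor along the spline.
; Tick turns the scene component toward the player camera as a billboard.
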(event `self.ReceiveBeginPlay`
  (bind _returnvalue (`PrimitiveComponent.CreateDynamicMaterialInstance` (`self.Plane`) 0 "/Game/GA/Materials/M_MaskedUnlit.M_MaskedUnlit" "None"))
  (bind _output_get (set `self.ColorMat` _returnvalue))
  (`MaterialInstanceDynamic.SetVectorParameterValue` _output_get "Color" (select `int` (`KismetMathLibrary.RandomIntegerInRange` 0 7) :`0` (struct :`R` 1.0 :`G` 0.014468 :`A` 1.0) :`1` (struct :`R` 1.0 :`B` 0.900793 :`A` 1.0) :`2` (struct :`G` 0.199193 :`B` 1.0 :`A` 1.0) :`3` (struct :`G` 0.718661 :`B` 1.0 :`A` 1.0) :`4` (struct :`G` 1.0 :`B` 0.254847 :`A` 1.0) :`5` (struct :`R` 0.104175 :`G` 1.0 :`A` 1.0) :`6` (struct :`R` 0.746613 :`G` 1.0 :`A` 1.0) :`7` (struct :`R` 1.0 :`G` 0.545587 :`A` 1.0) :!type "LinearColor Structure"))
  (`self.Move Object`))

(event `Move Object`
  (`TimelineComponent.SetPlayRate` (`self.MoveObjectT`) (/ 1.0 (/ (`SplineComponent.GetSplineLength` (`/Game/Interactif/1DTravel/BP_1DSpline.Spline` (`self.1DLine`))) (`self.Speed`))))
  (bind (_direction _alpha) (`Timeline|MoveObjectT` :!via `PlayFromStart`)
    (:`Update`
      (`self.K2_SetActorTransform` (`KismetMathLibrary.MakeTransform` (`SplineComponent.GetLocationAtDistanceAlongSpline` (`/Game/Interactif/1DTravel/BP_1DSpline.Spline` (`self.1DLine`)) (`KismetMathLibrary.Lerp` 0.0 (`SplineComponent.GetSplineLength` (`/Game/Interactif/1DTravel/BP_1DSpline.Spline` (`self.1DLine`))) _alpha) "World"))))
    (:`Finished`
      (`self.K2_DestroyActor`))))

(event `self.ReceiveTick`
  (params (DeltaSeconds :type "Float (single-precision)"))
  (bind _scene (`self.Scene`))
  (`SceneComponent.K2_SetWorldRotation` _scene (`KismetMathLibrary.FindLookAtRotation` (`SceneComponent.K2_GetComponentLocation` _scene) (`SceneComponent.K2_GetComponentLocation` (`PlayerCameraManager.TransformComponent` (`GameplayStatics.GetPlayerCameraManager` 0)))) false true))

(fn `UserConstructionScript`)