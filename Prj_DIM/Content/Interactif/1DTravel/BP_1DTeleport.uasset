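; One-shot trigger that moves the player out of 1D travel to an arrival point.
; When a BP_1DController overlaps the box, it stops that controller and, after a short delay, has its Player take control at the arrival point and rotation.
; An Eject1D flag selects either an eject cinematic, with a boss animation on any linked FightRoom, or a cut to an end camera that blends back to the player.
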(event `self.Box.OnComponentBeginOverlap`
  (params (OverlappedComponent :type "PrimitiveComponent Object Reference") (OtherActor :type "Actor Object Reference") (OtherComp :type "PrimitiveComponent Object Reference") (OtherBodyIndex :type Integer) (bFromSweep :type Boolean) (SweepResult :type "HitResult Structure (by ref)"))
  (bind _fightroom (`self.fightRoom`))
  (bind _asbp_1dcontroller (cast `/Game/Interactif/1DTravel/BP_1DController` OtherActor))
  (`/Engine/EditorBlueprintResources/StandardMacros.DoOnce` false
    (:`Completed`
      (bind _player (`/Game/Interactif/1DTravel/BP_1DController.Player` _asbp_1dcontroller))
      (set `self.Test` _player)
      (`/Game/Interactif/1DTravel/BP_1DController.StopControl` _asbp_1dcontroller)
      (`KismetSystemLibrary.Delay` 1.5)
      (`/Game/Player/BP_Player.TakeControl1D` _player (`self.ArrivalPoint`) (`self.ArrivalControlRot`))
      (if (`self.Eject1D`)
        (`/Game/Player/BP_Player.Eject1DCine` (`self.Test`))
        (`/Engine/EditorBlueprintResources/StandardMacros.IsValid` _fightroom
          (:`Is Valid`
            (`/Game/Interactif/AI/BP_FightRoom.Eject1DAnimBoss` _fightroom)))
        (else
          (`PlayerController.SetViewTargetWithBlend` (`GameplayStatics.GetPlayerController` 0) (`self.EndCamera`) 0.0 "VTBlend_Cubic" 0.5 false)
          (`PlayerController.SetViewTargetWithBlend` (`GameplayStatics.GetPlayerController` 0) _player 2.5 "VTBlend_Cubic" 0.5 false))))))

(fn `UserConstructionScript`)