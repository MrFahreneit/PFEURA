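; BP_Boss1D is a boss actor, filed under 1D Travel, that slides between two points and keeps facing the camera.
; It records its spawn location as PointA on BeginPlay.
; MoveBoss plays a timeline, rate-scaled by TimeMove, that lerps the actor from PointA to the current location of ActorPointB.
; Every tick it rotates its Scene component toward the player camera, billboard-style.
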(event `self.ReceiveBeginPlay`
  (set `self.PointA` (`self.K2_GetActorLocation`)))

(event `MoveBoss`
  (`TimelineComponent.SetPlayRate` (`self.MovePointA_B`) (/ 1.0 (`self.TimeMove`)))
  (bind (_direction _alpha) (`Timeline|MovePointA_B` :!via `PlayFromStart`)
    (:`Update`
      (`self.K2_SetActorLocation` (`KismetMathLibrary.VLerp` (`self.PointA`) (`self.K2_GetActorLocation` (`self.ActorPointB`)) _alpha)))))

(event `self.ReceiveTick`
  (params (DeltaSeconds :type "Float (single-precision)"))
  (bind _scene (`self.Scene`))
  (`SceneComponent.K2_SetWorldRotation` _scene (`KismetMathLibrary.FindLookAtRotation` (`SceneComponent.K2_GetComponentLocation` _scene) (`SceneComponent.K2_GetComponentLocation` (`PlayerCameraManager.TransformComponent` (`GameplayStatics.GetPlayerCameraManager` 0)))) false true))

(fn `UserConstructionScript`)