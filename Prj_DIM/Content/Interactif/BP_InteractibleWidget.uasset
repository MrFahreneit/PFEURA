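; BP_InteractibleWidget is an actor that fades an interaction prompt widget in and out.
; Its ShowActor event takes an On flag: true unhides the widget component and plays the WW_Interact Fade animation, while false plays it in reverse without re-hiding the component.
; Two DoOnce gates reset each other, so repeated calls with the same state do not restart the fade.
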(event `ShowActor`
  (params (`on?` :type Boolean))
  (bind _widget (`self.Widget`))
  (bind _returnvalue (`WidgetComponent.GetUserWidgetObject` _widget))
  (if `on?`
    (`/Engine/EditorBlueprintResources/StandardMacros.DoOnce` false :!label _label
      (:`Completed`
        (`SceneComponent.SetHiddenInGame` _widget (not `on?`) false)
        (bind _asww_interact (cast `/Game/HUD/WW_Interact` _returnvalue))
        (`UserWidget.PlayAnimation` _asww_interact (`/Game/HUD/WW_Interact.Fade` _asww_interact) 0.0 1 "Forward" 1.0 false)
        (goto _label_2 :!via `Reset`)))
    (else
      (`/Engine/EditorBlueprintResources/StandardMacros.DoOnce` false :!label _label_2
        (:`Completed`
          (bind _asww_interact_2 (cast `/Game/HUD/WW_Interact` _returnvalue))
          (`UserWidget.PlayAnimation` _asww_interact_2 (`/Game/HUD/WW_Interact.Fade` _asww_interact_2) 0.0 1 "Reverse" 1.0 false)
          (goto _label :!via `Reset`))))))

(fn `UserConstructionScript`)