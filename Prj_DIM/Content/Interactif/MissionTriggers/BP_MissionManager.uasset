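; BP_MissionManager is a placed trigger box that starts or completes a mission on the player's HUD.
; On the first player overlap, it either calls CompleteMission on the HUD widget when Completion is set, or updates the displayed mission.
; The update reads name and description from DT_Mission, using the MissionType enum's string as the row name.
; BeginPlay checks FightRoomLink's validity but does nothing with it.
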(event `self.ReceiveBeginPlay`
  (`/Engine/EditorBlueprintResources/StandardMacros.IsValid` (`self.FightRoomLink`)))

(event `self.Box.OnComponentBeginOverlap`
  (params (OverlappedComponent :type "PrimitiveComponent Object Reference") (OtherActor :type "Actor Object Reference") (OtherComp :type "PrimitiveComponent Object Reference") (OtherBodyIndex :type Integer) (bFromSweep :type Boolean) (SweepResult :type "HitResult Structure (by ref)"))
  (bind _asbp_player (cast `/Game/Player/BP_Player` OtherActor))
  (`/Engine/EditorBlueprintResources/StandardMacros.DoOnce` false
    (:`Completed`
      (if (`self.Completion`)
        (bind _hud_widget (`/Game/Player/BP_Player.HUD_Widget` _asbp_player))
        (`/Game/UI/Widgets/HUD/W_HUD.CompleteMission` _hud_widget)
        (else
          (bind _returnvalue (`|GetDataTableRow` "/Game/Interactif/MissionTriggers/DT_Mission.DT_Mission" (`KismetStringLibrary.Conv_StringToName` (`|GetEnumeratorNameAsString` (`self.MissionType`))))
            (:`then`
              (bind (_missiontype _missionname _description) (break `/Game/Interactif/MissionTriggers/S_Mission` _returnvalue))
              (`/Game/UI/Widgets/HUD/W_HUD.UpdateMission` _hud_widget _missionname _description))))))))

(fn `UserConstructionScript`)