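; BP_CollectWeapon is an interactive weapon pickup that grants the player a glove when collected.
; Its CurrentWeapon data table row sets the decal material in the construction script and on BeginPlay, which also stores the row as weapon stats.
; On collect, it calls ObtainGlove on the player, then destroys the BPCollectItem child actor and itself, without using the stored stats.
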(event `self.ReceiveBeginPlay`
  (bind (_currentweapon_datatable _currentweapon_rowname) (break `DataTableRowHandle` (`self.CurrentWeapon`)))
  (`parent.ReceiveBeginPlay`)
  (bind _returnvalue (`|GetDataTableRow` _currentweapon_datatable _currentweapon_rowname)
    (:`then`
      (set `self.WeaonStat` _returnvalue)
      (`DecalComponent.SetDecalMaterial` (`self.Decal`) (`.Decal_7_05C04F244FBE43AC007FE0BA66FC42E9` (break `/Game/Interactif/Collectable/S_WeaponStat` _returnvalue))))))

(event `self.DoCollectAction`
  (`parent.DoCollectAction`)
  (bind _asbp_player (cast `/Game/Player/BP_Player` (`GameplayStatics.GetPlayerCharacter` 0)))
  (`/Game/Player/BP_Player.Obtain Glove` _asbp_player)
  (`self.K2_DestroyActor` (`ChildActorComponent.ChildActor` (`self.BP_CollectItem`)))
  (`self.K2_DestroyActor`))

(event `/Game/Interactif/BPI_ActorInteract.StartEventInteract`
  (params (value :type Integer))
  (`parent.StartEventInteract` value))

(fn `UserConstructionScript`
  (bind (_currentweapon_datatable _currentweapon_rowname) (break `DataTableRowHandle` (`self.CurrentWeapon`)))
  (`parent.UserConstructionScript`)
  (bind _returnvalue (`|GetDataTableRow` _currentweapon_datatable _currentweapon_rowname)
    (:`then`
      (`DecalComponent.SetDecalMaterial` (`self.Decal`) (`.Decal_7_05C04F244FBE43AC007FE0BA66FC42E9` (break `/Game/Interactif/Collectable/S_WeaponStat` _returnvalue))))))