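; BP_ZoneKiller is a kill volume in the checkpoint system that respawns the player on contact.
; On BeginPlay it caches the GI_MasterInst game instance and the GM_gameplay game mode, though only the game mode is used afterward.
; When a BP_Player or BP_2DPlayer begins overlapping its Box component, it calls RespawnPlayer on the game mode, ignoring all other actors.
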(event `self.ReceiveBeginPlay`
  (bind _asgi_master_inst (cast `/Game/Player/GI_MasterInst` (`GameplayStatics.GetGameInstance`)))
  (set `self.As GI Master Inst` _asgi_master_inst)
  (bind _asgm_gameplay (cast `/Game/Player/GM_gameplay` (`GameplayStatics.GetGameMode`)))
  (set `self.As GM Gameplay` _asgm_gameplay))

(event `self.Box.OnComponentBeginOverlap`
  (params (OverlappedComponent :type "PrimitiveComponent Object Reference") (OtherActor :type "Actor Object Reference") (OtherComp :type "PrimitiveComponent Object Reference") (OtherBodyIndex :type Integer) (bFromSweep :type Boolean) (SweepResult :type "HitResult Structure (by ref)"))
  (cast `/Game/Player/BP_Player` OtherActor
    (:`then`
      _)
    (:`CastFailed`
      (cast `/Game/Player/2DPlayer/BP_2DPlayer` OtherActor)))
  (`/Game/Player/GM_gameplay.RespawnPlayer` (`self.As GM Gameplay`)))

(fn `UserConstructionScript`)