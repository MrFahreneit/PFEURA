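; BP_BGMTrigger is a trigger volume that changes background music when a 3D or 2D player overlaps its box.
; It can also fire one tick after BeginPlay, and TriggerOnce gates overlap triggering through a DoOnce.
; TriggerBGM forwards the configured track and fade settings to the GM_gameplay game mode's BGMManager, which plays new music, plays it without overlap, or stops it according to PlayType.
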(event `self.ReceiveBeginPlay`
  (`KismetSystemLibrary.DelayUntilNextTick`)
  (if (`self.TriggerOnStart`)
    (`self.TriggerBGM`)))

(event `self.Box.OnComponentBeginOverlap`
  (params (OverlappedComponent :type "PrimitiveComponent Object Reference") (OtherActor :type "Actor Object Reference") (OtherComp :type "PrimitiveComponent Object Reference") (OtherBodyIndex :type Integer) (bFromSweep :type Boolean) (SweepResult :type "HitResult Structure (by ref)"))
  (cast `/Game/Player/BP_Player` OtherActor
    (:`then`
      _)
    (:`CastFailed`
      (cast `/Game/Player/2DPlayer/BP_2DPlayer` OtherActor)))
  (if (`self.TriggerOnce`)
    (`/Engine/EditorBlueprintResources/StandardMacros.DoOnce` false
      (:`Completed`
        _)))
  (`self.TriggerBGM`))

(fn `TriggerBGM`
  (bind _asgm_gameplay (cast `/Game/Player/GM_gameplay` (`GameplayStatics.GetGameMode`)))
  (switch `/Game/ScoresAndSountrack/E_BGMPlayType` (`self.PlayType`)
    (:`NewEnumerator1`
      (bind _bgmmanager (`/Game/Player/GM_gameplay.BGMManager` _asgm_gameplay))
      (`/Game/ScoresAndSountrack/BP_BGMManager.PlayNewBGM` _bgmmanager (`self.FadeOutDuration`) (`self.BGMToPlay`) (`self.FadeInDuration`)))
    (:`NewEnumerator2`
      (`/Game/ScoresAndSountrack/BP_BGMManager.PlayNewBGMNoOverlap` _bgmmanager (`self.FadeOutDuration`) (`self.BGMToPlay`) (`self.FadeInDuration`) (`self.NewFadeInDelay`)))
    (:`NewEnumerator3`
      (`/Game/ScoresAndSountrack/BP_BGMManager.StopBGM` _bgmmanager (`self.FadeOutDuration`)))))

(fn `UserConstructionScript`)