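; Window prop Blueprint that randomizes its mesh, wood color and glass glow in the Construction Script, with no active runtime logic.
; A random index picks the mesh from AllWindowMesh and selects a vector whose X and Y give its wood and glass material slots.
; Dynamic material instances on those slots receive a random palette color and a random EmissiveIntensity.
; Two older per-mesh branch chains remain unconnected and never run.
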(fn `UserConstructionScript`
  (bind _vector_x (`KismetMathLibrary.BreakVector2D` (`self.vector`)))
  (bind _index (`self.index`))
  (bind (_vector_x_2 _vector_y) (`KismetMathLibrary.BreakVector2D` (`self.vector`)))
  (set `self.index` (`.OutIndex` (`KismetArrayLibrary.Array_Random` (`self.AllWindowMesh`))))
  (`StaticMeshComponent.SetStaticMesh` (`self.SM_Fenetre_1`) (`|GetArrayItem` (`self.AllWindowMesh`) _index))
  (set `self.vector` (select `int` _index :`0` (0.0 1.0) :`1` (1.0 2.0) :`2` (1.0 2.0) :`3` (0.0 1.0) :!type "Vector2D Structure"))
  (bind _returnvalue (`PrimitiveComponent.CreateDynamicMaterialInstance` (`self.SM_Fenetre_1`) (`KismetMathLibrary.FTrunc` _vector_x) "/Game/GA/Materials/Environment/MI_Wood.MI_Wood" "None"))
  (bind _output_get (set `self.mat` _returnvalue))
  (`MaterialInstanceDynamic.SetVectorParameterValue` _output_get "Color" (`KismetArrayLibrary.Array_Random` (`|MakeArray` (struct :`R` 0.4375 :`G` 0.274972 :`B` 0.198242 :`A` 1.0) (struct :`R` 0.328125 :`G` 0.215481 :`B` 0.091889 :`A` 1.0) (struct :`R` 0.651042 :`G` 0.315348 :`B` 0.319863 :`A` 1.0) (struct :`R` 0.4375 :`G` 0.182954 :`B` 0.086589 :`A` 1.0) (struct :`R` 0.395833 :`G` 0.259194 :`B` 0.119575 :`A` 1.0) :!type "LinearColor Structure")))
  (bind _returnvalue_2 (`PrimitiveComponent.CreateDynamicMaterialInstance` (`self.SM_Fenetre_1`) (`KismetMathLibrary.FTrunc` _vector_y) "/Game/GA/Materials/Environment/MI_VitreFenetres_01.MI_VitreFenetres_01" "None"))
  (set `self.Intensity` _returnvalue_2)
  (`MaterialInstanceDynamic.SetScalarParameterValue` _returnvalue_2 "EmissiveIntensity" (`KismetMathLibrary.RandomFloatInRange` 0.0 5.0)))