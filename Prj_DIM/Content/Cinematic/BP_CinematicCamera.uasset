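; BP_CinematicCamera is a placed camera actor that plays an intro-style cinematic along waypoint actors when its Start flag is set.
; On BeginPlay it disables player input, forces the player's 2D check, disables 2D interaction and becomes the view target.
; A recursive timeline event lerps location and rotation through Points, using per-point travel and wait times.
; After the last point, it blends back to the player and re-enables pawn input.
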(event `self.ReceiveBeginPlay`
  (bind _returnvalue (`GameplayStatics.GetPlayerCharacter` 0))
  (bind _returnvalue_2 (`GameplayStatics.GetPlayerController` 0))
  (if (`self.start`)
    (bind _asbp_player (cast `/Game/Player/BP_Player` (`GameplayStatics.GetPlayerCharacter` 0)))
    (`self.DisableInput` (`GameplayStatics.GetPlayerController` 0) null)
    (`self.DisableInput` _asbp_player null)
    (`KismetSystemLibrary.Delay` 0.1)
    (`/Game/Player/BP_Player.Force2DCheck` _asbp_player)
    (if (`self.start`)
      (`|ExecutionSequence`
        (:`then_0`
          (`PlayerController.SetViewTargetWithBlend` (`GameplayStatics.GetPlayerController` 0) self 0.0 "VTBlend_Linear" 0.0 false)
          (`self.NewCamMovement`)
          (bind _asbp_player_2 (cast `/Game/Player/BP_Player` _returnvalue))
          (`/Game/Player/BP_Player.SetDisable2DInteract` _asbp_player_2 true)
          (`self.DisableInput` _returnvalue (`GameplayStatics.GetPlayerController` 0)))
        (:`then_1`
          (`self.DisableInput` _returnvalue_2 _returnvalue_2)
          (`self.DisableInput` (`Controller.K2_GetPawn` _returnvalue_2) _returnvalue_2))))))

(event `NewCamMovement`
  (bind _returnvalue (`GameplayStatics.GetPlayerController` 0))
  (bind _currentindex (`self.currentIndex`))
  (bind _points (`self.Points`))
  (bind (_pointa_location _pointa_rotation) (`KismetMathLibrary.BreakTransform` (`self.PointA`)))
  (bind (_pointb_location _pointb_rotation) (`KismetMathLibrary.BreakTransform` (`self.PointB`)))
  (set `self.PointA` (`self.GetTransform`))
  (if (> _currentindex (`KismetArrayLibrary.Array_LastIndex` _points))
    (`PlayerController.SetViewTargetWithBlend` (`GameplayStatics.GetPlayerController` 0) (`GameplayStatics.GetPlayerCharacter` 0) 0.5 "VTBlend_Linear" 0.0 false)
    (`KismetSystemLibrary.Delay` 0.6)
    (`self.EnableInput` (`Controller.K2_GetPawn` _returnvalue) _returnvalue)
    (else
      (set `self.PointB` (`self.GetTransform` (`|GetArrayItem` _points _currentindex)))
      (`TimelineComponent.SetPlayRate` (`self.MoveCamera`) (/ 1.0 (`|GetArrayItem` (`self.Tim`) _currentindex)))
      (bind (_direction _alpha) (`Timeline|MoveCamera` :!via `PlayFromStart`)
        (:`Update`
          (`self.K2_SetActorTransform` (`KismetMathLibrary.MakeTransform` (`KismetMathLibrary.VLerp` _pointa_location _pointb_location _alpha) (`KismetMathLibrary.RLerp` _pointa_rotation _pointb_rotation _alpha true))))
        (:`Finished`
          (`KismetSystemLibrary.Delay` (`|GetArrayItem` (`self.waitTime`) _currentindex))
          (`/Engine/EditorBlueprintResources/StandardMacros.IncrementInt` (`self.currentIndex`)
            (:`  `
              (`self.NewCamMovement`))))))))

(fn `UserConstructionScript`)