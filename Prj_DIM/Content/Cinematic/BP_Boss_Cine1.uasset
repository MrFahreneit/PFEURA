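; Boss cinematic actor that plays a one-shot boss animation when the 2D player first enters its trigger box.
; A DoOnce-guarded box overlap calls StartAnim, which starts the montage-free animation on the skeletal mesh and reveals it two ticks later, then hides it again after a fixed delay.
; A parallel sequence branch fires shoot and fall-down legacy camera shakes on the player camera shortly after the start.
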(event `StartAnim`
  (bind _returnvalue (`GameplayStatics.GetPlayerCameraManager` 0))
  (bind _skeletalmesh (`self.SkeletalMesh`))
  (`SkeletalMeshComponent.PlayAnimation` _skeletalmesh "/Game/GA/Skeletal/Boss/A_Boss_Cine1.A_Boss_Cine1" false)
  (`|ExecutionSequence`
    (:`then_0`
      (`KismetSystemLibrary.DelayUntilNextTick`)
      (`KismetSystemLibrary.DelayUntilNextTick`)
      (`SceneComponent.SetVisibility` _skeletalmesh true false)
      (`SceneComponent.SetHiddenInGame` _skeletalmesh false false)
      (`KismetSystemLibrary.Delay` 6.0)
      (`SceneComponent.SetHiddenInGame` _skeletalmesh true false)
      (`SceneComponent.SetVisibility` _skeletalmesh false false))
    (:`then_1`
      (`KismetSystemLibrary.Delay` 0.75)
      (`LegacyCameraShake.StartLegacyCameraShake` _returnvalue "/Game/Player/Shakes/CS_Shoot.CS_Shoot_C" 15.0)
      (`KismetSystemLibrary.DelayUntilNextTick`)
      (`LegacyCameraShake.StartLegacyCameraShake` _returnvalue "/Game/Player/Shakes/CS_BossFallDown.CS_BossFallDown_C"))))

(event `self.Box.OnComponentBeginOverlap`
  (params (OverlappedComponent :type "PrimitiveComponent Object Reference") (OtherActor :type "Actor Object Reference") (OtherComp :type "PrimitiveComponent Object Reference") (OtherBodyIndex :type Integer) (bFromSweep :type Boolean) (SweepResult :type "HitResult Structure (by ref)"))
  (cast `/Game/Player/2DPlayer/BP_2DPlayer` OtherActor)
  (`/Engine/EditorBlueprintResources/StandardMacros.DoOnce` false
    (:`Completed`
      (`self.StartAnim`))))

(fn `UserConstructionScript`)