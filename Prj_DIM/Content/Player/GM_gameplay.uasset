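; GM_gameplay is the gameplay game mode that handles checkpoint respawning for the player.
; On BeginPlay it caches the master game instance and player, seeding the instance's checkpoint transform with the player's starting transform if it is still zero.
; RespawnPlayer teleports the player to that stored transform and resets control rotation to the checkpoint yaw with a fixed downward pitch.
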(event `self.ReceiveBeginPlay`
  (bind (_checkpointtransform_location _checkpointtransform_rotation) (`KismetMathLibrary.BreakTransform` (`/Game/Player/GI_MasterInst.CheckPointTransform` (`self.As GI Master Inst`))))
  (bind _asgi_master_inst (cast `/Game/Player/GI_MasterInst` (`GameplayStatics.GetGameInstance`)))
  (set `self.As GI Master Inst` _asgi_master_inst)
  (bind _asbp_player (cast `/Game/Player/BP_Player` (`GameplayStatics.GetPlayerCharacter` 0)))
  (bind _output_get (set `self.As BP Player` _asbp_player))
  (if (and (== _checkpointtransform_location (0.0 0.0 0.0) :`ErrorTolerance` 0.1) (== _checkpointtransform_rotation (struct) :`ErrorTolerance` 0.1))
    (set `/Game/Player/GI_MasterInst.CheckPointTransform` (`self.GetTransform` _output_get) (`self.As GI Master Inst`))))

(event `RespawnPlayer`
  (bind (_checkpointtransform_location _checkpointtransform_rotation) (`KismetMathLibrary.BreakTransform` (`/Game/Player/GI_MasterInst.CheckPointTransform` (`self.As GI Master Inst`))))
  (`self.K2_SetActorTransform` (`self.As BP Player`) (`KismetMathLibrary.MakeTransform` _checkpointtransform_location _checkpointtransform_rotation) false true)
  (`Controller.SetControlRotation` (`GameplayStatics.GetPlayerController` 0) (`KismetMathLibrary.MakeRotator` 0.0 -45.0 (.yaw _checkpointtransform_rotation))))

(fn `UserConstructionScript`)