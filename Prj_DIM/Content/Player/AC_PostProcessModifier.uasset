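; Player actor component that locates the level's PostProcessVolume, apparently as groundwork for modifying post-processing at runtime.
; On BeginPlay it loops over all such volumes, storing each in a variable so the last one wins, and prints a red on-screen warning if there are several.
; Unconnected nodes for creating a dynamic material instance and adding a weighted blendable never run, so no effect is applied.
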(event `self.ReceiveBeginPlay`
  (bind _outactors (`GameplayStatics.GetAllActorsOfClass` "/Script/Engine.PostProcessVolume"))
  (for (_array_element _array_index) _outactors
    (set `self.PostProcessVolume` _array_element)
    (if (> _array_index 0)
      (`KismetSystemLibrary.PrintString` "MULTIPLE POST PROCESS VOLUME DETECTED" true false (struct :`R` 1.0 :`A` 1.0) 20.0))))