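; Test player Blueprint for combat that layers battle input on top of its parent class.
; BeginPlay runs the parent logic, then hides the HUD widget.
; The light attack Enhanced Input action calls AttackLight on the ACBattleSystem component when it starts.
; Heavy, charged light and charged heavy attack calls are present but not wired to any event.
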(event `self.ReceiveBeginPlay`
  (`parent.ReceiveBeginPlay`)
  (`Widget.SetVisibility` (`self.HUD_Widget`) "Hidden"))

(event `self.ReceiveActorBeginOverlap`
  (params (OtherActor :type "Actor Object Reference")))

(event `self.ReceiveTick`
  (params (DeltaSeconds :type "Float (single-precision)"))
  (`parent.ReceiveTick` DeltaSeconds))

(event `EnhancedInput|/Game/ThirdPerson/Input/Actions/IA_AttackLight`
  (params (ActionValue :type Boolean) (ElapsedSeconds :type "Float (double-precision)") (TriggeredSeconds :type "Float (double-precision)") (InputAction :type "InputAction Object Reference" :default "/Game/ThirdPerson/Input/Actions/IA_AttackLight.IA_AttackLight"))
  ;[1 1 1] Combat Input
  (:`Started`
    (`/Game/Player/BattleSystem/AC_BattleSystem.AttackLight` (`self.AC_BattleSystem`))))

(event `EnhancedInput|/Game/ThirdPerson/Input/Actions/IA_AttackLightCharged`
  (params (ActionValue :type Boolean) (ElapsedSeconds :type "Float (double-precision)") (TriggeredSeconds :type "Float (double-precision)") (InputAction :type "InputAction Object Reference" :default "/Game/ThirdPerson/Input/Actions/IA_AttackLightCharged.IA_AttackLightCharged"))
  ;[1 1 1] Combat Input
)

(event `EnhancedInput|/Game/ThirdPerson/Input/Actions/IA_AttackHeavyCharged`
  (params (ActionValue :type Boolean) (ElapsedSeconds :type "Float (double-precision)") (TriggeredSeconds :type "Float (double-precision)") (InputAction :type "InputAction Object Reference" :default "/Game/ThirdPerson/Input/Actions/IA_AttackHeavyCharged.IA_AttackHeavyCharged"))
  ;[1 1 1] Combat Input
)

(event `EnhancedInput|/Game/ThirdPerson/Input/Actions/IA_AttackHeavy`
  (params (ActionValue :type Boolean) (ElapsedSeconds :type "Float (double-precision)") (TriggeredSeconds :type "Float (double-precision)") (InputAction :type "InputAction Object Reference" :default "/Game/ThirdPerson/Input/Actions/IA_AttackHeavy.IA_AttackHeavy"))
  ;[1 1 1] Combat Input
)

(fn `UserConstructionScript`
  (`parent.UserConstructionScript`))