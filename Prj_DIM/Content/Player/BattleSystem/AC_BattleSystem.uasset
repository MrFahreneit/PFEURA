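; Character component that runs the player's melee combo combat, with light, heavy, charged, running and aerial attacks.
; Inputs buffer the next attack from DT_Attack combo links, and TryNextAttack plays its montage when free.
; Montage notifies drive attack state, gravity, charge damage and sphere-trace hitboxes that damage BPI_Damageable actors.
; It also keeps a timed HUD combo meter, a ground check for aerial heavies and a one-shot debug toggle.
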(event `self.ReceiveBeginPlay`
  (bind _ascharacter (cast `Character` (`self.GetOwner`)))
  (set `self.OwnerCharacter` _ascharacter)
  (set `self.OwnerMovementComponent` (`Actor.GetComponentByClass` (`self.OwnerCharacter`) "/Script/Engine.CharacterMovementComponent"))
  (set `self.DefaultGravityScale` (`CharacterMovementComponent.GravityScale` (`self.OwnerMovementComponent`))))

(event `ClearBufferTimer`
  ;[1 1 1] Clear Timers
  (`KismetSystemLibrary.RetriggerableDelay` 0.4)
  (`self.ClearBuffer`))

(event `ClearComboTimer`
  ;[1 1 1] Clear Timers
  (`KismetSystemLibrary.RetriggerableDelay` 0.4)
  (`self.ClearCombo`))

(event `AttackLight`
  ;[1 1 1] Inputs
  (`self.BufferAttack` "NewEnumerator4"))

(event `AttackHeavy`
  ;[1 1 1] Inputs
  (`self.BufferAttack` "NewEnumerator0"))

(event `LightChargedRelease`
  ;[1 1 1] Inputs
  (if (`|EnumEquality` (`self.CurrentAttack`) "NewEnumerator11")
    (set `self.LightChargedBuffer` true)
    (`self.TryNextAttack` :!label _label)))

(event `PlayAttackAnimation`
  (params (AttackName :type "/Game/Player/BattleSystem/E_AttackName Enum" :default "NewEnumerator4"))
  (bind _currentattack (`self.CurrentAttack`))
  (bind (_attackname _damage _hitboxtype _hitboxrange _launchforce _animation _canbreakguard _cantrigger2d _canairlaunch _caninputrotation _magnettoenemy) (break `/Game/Player/BattleSystem/S_Attack` (`self.GetAttackData` AttackName)))
  (if (or (`self.LightChargedBuffer`) (`self.HeavyChargedBuffer`))
    (set `self.LightChargedBuffer` false)
    (set `self.HeavyChargedBuffer` false))
  (if _caninputrotation
    (set `self.InstantRotate` true)
    (`KismetSystemLibrary.Delay` 0.0)
    (set `self.InstantRotate` false))
  (if _magnettoenemy
    (set `self.IsSnapping` true)
    (`KismetSystemLibrary.Delay` 0.0)
    (set `self.IsSnapping` false))
  (bind _notifyname (`|PlayMontage` (`Character.Mesh` (`self.OwnerCharacter`)) _animation)
    (:`then`
      (set `self.CurrentAttack` AttackName)
      (if (and (`|EnumInequality` (`self.GetMovementMode`) "MOVE_Walking") (`|EnumInequality` _currentattack "NewEnumerator19") (`|EnumInequality` _currentattack "NewEnumerator22"))
        (set `MovementComponent.Velocity` (0.0 0.0 420.0) (`self.OwnerMovementComponent`))
        (`KismetSystemLibrary.Delay` 0.1)
        (`CharacterMovementComponent.SetMovementMode` (`self.OwnerMovementComponent`) "MOVE_None" 0)
        (`KismetSystemLibrary.RetriggerableDelay` 0.2)
        (`self.ReEnableFalling` true)))
    (:`OnNotifyBegin`
      (`self.OnBeginNotif` _notifyname))))

(event `HeavyChargedRelease`
  ;[1 1 1] Inputs
  (if (`|EnumEquality` (`self.CurrentAttack`) "NewEnumerator18")
    (set `self.HeavyChargedBuffer` true)
    (goto _label)))

(event `AttackLightCharged`
  ;[1 1 1] Inputs
  (if (`|EnumInequality` (`.AttackName_27_53FD94BD4B74A85466997584711663E6` (break `/Game/Player/BattleSystem/S_Attack` (`self.GetAttackData` (`self.CurrentAttack`)))) "NewEnumerator11")
    (`self.BufferAttack` "NewEnumerator1")))

(event `AttackHeavyCharged`
  ;[1 1 1] Inputs
  (if (`|EnumInequality` (`.AttackName_27_53FD94BD4B74A85466997584711663E6` (break `/Game/Player/BattleSystem/S_Attack` (`self.GetAttackData` (`self.CurrentAttack`)))) "NewEnumerator18")
    (`self.BufferAttack` "NewEnumerator2")))

(event `DashStart`
  ;[1 1 1] Inputs
  (set `self.IsDash` true))

(event `DashEnd`
  (params (CD :type "Float (double-precision)"))
  ;[1 1 1] Inputs
  (`KismetSystemLibrary.Delay` CD)
  (set `self.IsDash` false))

(event `Block`
  (params (Enable :type Boolean))
  ;[1 1 1] Inputs
)

(event `Enter4DState`
  ;[1 1 1] Inputs
)

(event `self.ReceiveTick`
  (params (DeltaSeconds :type "Float (single-precision)")))

(event `Exit4DState`
  ;[1 1 1] Inputs
)

(fn `BufferAttack`
  (params (AttackType :type "/Game/Player/BattleSystem/E_AttackType Enum" :default "NewEnumerator4"))
  (bind _asbp_player (cast `/Game/Player/BP_Player` (`self.OwnerCharacter`) :!pure true))
  (bind (_attackname _damage _hitboxtype _hitboxrange _launchforce _animation _canbreakguard _cantrigger2d _canairlaunch _caninputrotation _magnettoenemy _airtime _nextlight _nextheavy _nextlightcharged _nextheavycharged) (break `/Game/Player/BattleSystem/S_Attack` (`self.GetAttackData` (`self.CurrentAttack`))))
  (if (not (`|EnumInequality` (`self.GetMovementMode`) "MOVE_Walking"))
    (if (or (`/Game/Player/BP_Player.IsRunning` _asbp_player) (`self.IsDash`))
      (`self.BufferCheck` (select `/Game/Player/BattleSystem/E_AttackType` (`local.AttackType`) :`NewEnumerator4` "NewEnumerator10" :`NewEnumerator0` "NewEnumerator17" :`NewEnumerator1` "NewEnumerator4" :`NewEnumerator2` "NewEnumerator4" :!type "/Game/Player/BattleSystem/E_AttackName Enum") ; Running Buffer
        (:`Valid`
          (`/Game/Player/BP_Player.SetRun` _asbp_player false)))
      (else
        (`self.BufferCheck` (select `/Game/Player/BattleSystem/E_AttackType` (`local.AttackType`) :`NewEnumerator4` _nextlight :`NewEnumerator0` _nextheavy :`NewEnumerator1` _nextlightcharged :`NewEnumerator2` _nextheavycharged) ; Usual Buffer
          (:`Valid`
            _))))
    (else
      (`self.BufferCheck` (select `/Game/Player/BattleSystem/E_AttackType` (`local.AttackType`) :`NewEnumerator4` (`.NextLight_35_854AD1A1499C2935DBCFBDA247AEB8C9` (break `/Game/Player/BattleSystem/S_Attack` (`self.GetAttackData` (`self.CurrentAttack`)))) :`NewEnumerator0` "NewEnumerator19" :`NewEnumerator1` "NewEnumerator4" :`NewEnumerator2` "NewEnumerator4") ; Buffer Aerial
        (:`Valid`
          (if (`|EnumEquality` (`self.BufferedAttack`) "NewEnumerator19")
            (`KismetSystemLibrary.K2_SetTimer` null "CheckForGround" 0.01 true))))))
  (`self.ClearBufferTimer`)
  (`self.TryNextAttack`))

(fn `ChargeDamage`
  (set `self.BonusDamage` (`KismetMathLibrary.SelectFloat` (+ (`self.BonusDamage`) 1.0) 40.0 (< (`self.BonusDamage`) 40.0))))

(fn `CheckForGround`
  (bind _ownercharacter (`self.OwnerCharacter`))
  (bind _returnvalue (`Actor.K2_GetActorLocation` _ownercharacter))
  (bind _returnvalue_2 (`Actor.GetActorUpVector` _ownercharacter))
  (bind (_outhit _returnvalue_3) (`KismetSystemLibrary.SphereTraceSingle` (+ _returnvalue (* _returnvalue_2 -70.0)) (+ _returnvalue (* _returnvalue_2 -70.0)) 30.0 "TraceTypeQuery1"))
  (if _returnvalue_3
    (`KismetSystemLibrary.K2_ClearTimer` null "CheckForGround")
    (`self.PlayAttackAnimation` "NewEnumerator22")))

(fn `ClearBuffer`
  (set `self.BufferedAttack` "NewEnumerator4"))

(fn `ClearCombo`
  (set `self.CurrentAttack` "NewEnumerator4"))

(fn `DEBUGAttack`
  (bind _ownercharacter (`self.OwnerCharacter`))
  (bind _returnvalue (+ (`Actor.K2_GetActorLocation` _ownercharacter) (* (`Actor.GetActorForwardVector` _ownercharacter) 100.0)))
  (bind _outhits (`KismetSystemLibrary.SphereTraceMulti` :`Start` _returnvalue :`End` _returnvalue :`Radius` 75.0 :`TraceChannel` "TraceTypeQuery4" :`DrawDebugType` "ForDuration"))
  (for _array_element _outhits
    (bind (_bblockinghit _binitialoverlap _time _distance _location _impactpoint _normal _impactnormal _physmat _hitactor _hitcomponent) (`GameplayStatics.BreakHitResult` _array_element))
    (bind (_asai_master _bsuccess) (cast `/Game/Interactif/AI/AI_Master` _hitactor :!pure true))
    (if (and (`KismetSystemLibrary.DoesImplementInterface` _hitactor "/Game/Interactif/AI/BPI_Damageable.BPI_Damageable_C") (select `bool` _bsuccess :`false` true :`true` (== _hitcomponent (`Character.CapsuleComponent` _asai_master))))
      (message `/Game/Interactif/AI/BPI_Damageable.START_TAKE_DAMAGE` _hitactor null 15 30.0 false (0.0 0.0) false false false 0.0 0.0 "NewEnumerator0"))))

(fn `DecreaseComboMeterTimer`
  (bind _output_get (set `self.ComboTimer` (- (`self.ComboTimer`) (/ (/ (`self.ComboTimerMax`) (`self.ComboHoldTime`)) 20.0))))
  (if (<= _output_get 0.0)
    (`KismetSystemLibrary.K2_ClearTimer` null "DecreaseComboMeterTimer")
    (`self.ResetComboMeter`)
    (set `self.ComboTimer` 0.0)))

(fn `DmgHitActors`
  (params (ActorsHit :type "Array of Actor Object Reference") (Damage :type Integer) (`Poise(Debug)` :type "Float (double-precision)") (`Launch?` :type Boolean) (LaunchForce :type "Vector2D Structure") (CanBreakGuard :type Boolean) (isA2DLaunch :type Boolean) (CanAirLaunch :type Boolean) (AirTime :type "Float (double-precision)") (HitFreezeTime :type "Float (double-precision)") (HitType :type "/Game/Interactif/AI/Enum_HitType Enum" :default "NewEnumerator0"))
  (bind _returnvalue (select `bool` (`self.OneShot`) :`false` (+ Damage (`KismetMathLibrary.FTrunc` (`self.BonusDamage`))) :`true` 999999))
  (for _array_element ActorsHit
    (if (`KismetSystemLibrary.DoesImplementInterface` _array_element "/Game/Interactif/AI/BPI_Damageable.BPI_Damageable_C")
      (`KismetSystemLibrary.PrintString` (`KismetStringLibrary.Conv_IntToString` _returnvalue) true false)
      (message `/Game/Interactif/AI/BPI_Damageable.START_TAKE_DAMAGE` _array_element self _returnvalue `Poise(Debug)` `Launch?` LaunchForce CanBreakGuard isA2DLaunch CanAirLaunch AirTime HitFreezeTime HitType)
      (`KismetSystemLibrary.K2_ClearTimer` null "ChargeDamage")
      (set `self.BonusDamage` 0.0))))

(fn `GetAttackData`
  (params (AttackName :type "/Game/Player/BattleSystem/E_AttackName Enum" :default "NewEnumerator4"))
  (returns (AttackData :type "/Game/Player/BattleSystem/S_Attack Structure") (IsValid :type Boolean))
  (bind _returnvalue (`|GetDataTableRow` "/Game/Player/BattleSystem/DT_Attack.DT_Attack" (`KismetStringLibrary.Conv_StringToName` (`|GetEnumeratorNameAsString` AttackName)))
    (:`then`
      (return _returnvalue true))
    (:`RowNotFound`
      (return (struct) false))))

(fn `GetMovementMode`
  (returns (`Movement Mode` :type "EMovementMode Enum"))
  (return (`CharacterMovementComponent.MovementMode` (`self.OwnerMovementComponent`))))

(fn `IncrementComboMeter`
  (`/Engine/EditorBlueprintResources/StandardMacros.IncrementInt` (`self.Combo`)
    (:`  `
      (set `self.ComboTimer` (`self.ComboTimerMax`))
      (`KismetSystemLibrary.K2_SetTimer` null "DecreaseComboMeterTimer" 0.05 true)
      (bind _asbp_player (cast `/Game/Player/BP_Player` (`self.OwnerCharacter`)))
      (bind _w_combometer (`/Game/UI/Widgets/HUD/W_HUD.W_ComboMeter` (`/Game/Player/BP_Player.HUD_Widget` _asbp_player)))
      (if (`/Game/UI/Widgets/ComboMeter/W_ComboMeter.isInCombo?` _w_combometer)
        (`/Game/UI/Widgets/ComboMeter/W_ComboMeter.UpdateCombo` _w_combometer (`self.Combo`))
        (else
          (`/Game/UI/Widgets/ComboMeter/W_ComboMeter.StartCombo` _w_combometer))))))

(fn `OnBeginNotif`
  (params (Selection :type Name))
  (switch `name` Selection
    (:`AnimStart`
      (set `self.IsAttacking` true)
      (`self.ClearBuffer`))
    (:`Hitbox_L`
      (`self.SpawnHitbox` "NewEnumerator0"))
    (:`Hitbox_R`
      (`self.SpawnHitbox` "NewEnumerator1"))
    (:`AttackStop`
      (set `self.IsAttacking` false)
      (`self.TryNextAttack`))
    (:`AnimEnd`
      (`self.ClearCombo`))
    (:`DisableGravity`
      (`CharacterMovementComponent.SetMovementMode` (`self.OwnerMovementComponent`) "MOVE_Flying" 0))
    (:`EnableGravity`
      (`CharacterMovementComponent.SetMovementMode` (`self.OwnerMovementComponent`) "MOVE_Falling" 0))
    (:`ChargeDamage`
      (`KismetSystemLibrary.K2_SetTimer` null "ChargeDamage" 0.1 true))))

(fn `ReEnableFalling`
  (params (ByMovementMode :type Boolean))
  (if ByMovementMode
    (`CharacterMovementComponent.SetMovementMode` (`self.OwnerMovementComponent`) "MOVE_Falling" 0)
    (else
      (set `CharacterMovementComponent.GravityScale` (`self.DefaultGravityScale`) (`self.OwnerMovementComponent`)))))

(fn `ResetComboMeter`
  (set `self.Combo` 0)
  (bind _asbp_player (cast `/Game/Player/BP_Player` (`self.OwnerCharacter`)))
  (`/Game/UI/Widgets/ComboMeter/W_ComboMeter.FinishedCombo` (`/Game/UI/Widgets/HUD/W_HUD.W_ComboMeter` (`/Game/Player/BP_Player.HUD_Widget` _asbp_player))))

(fn `SpawnHitbox`
  (params (HitType :type "/Game/Interactif/AI/Enum_HitType Enum" :default "NewEnumerator0"))
  (locals (GroundedEnemies :type "Array of Actor Object Reference"))
  (bind _ownercharacter (`self.OwnerCharacter`))
  (bind _ownercharacter_2 (`self.OwnerCharacter`))
  (bind _returnvalue (`Actor.K2_GetActorLocation` _ownercharacter_2))
  (bind _returnvalue_2 (`Actor.GetActorForwardVector` _ownercharacter_2))
  (bind _returnvalue_3 (`Actor.GetActorRightVector` _ownercharacter))
  (bind _returnvalue_4 (`Actor.K2_GetActorLocation` (`self.OwnerCharacter`)))
  (bind (_attackname _damage _hitboxtype _hitboxrange _launchforce _animation _canbreakguard _cantrigger2d _canairlaunch _caninputrotation _magnettoenemy _airtime) (break `/Game/Player/BattleSystem/S_Attack` (`self.GetAttackData` (`self.CurrentAttack`))))
  (bind (_attackname_2 _damage_2 _hitboxtype_2 _hitboxrange_2 _launchforce_2 _animation_2 _canbreakguard_2 _cantrigger2d_2 _canairlaunch_2 _caninputrotation_2 _magnettoenemy_2 _airtime_2) (break `/Game/Player/BattleSystem/S_Attack` (`self.GetAttackData` (`self.CurrentAttack`))))
  (bind (_attackname_3 _damage_3 _hitboxtype_3 _hitboxrange_3 _launchforce_3 _animation_3 _canbreakguard_3 _cantrigger2d_3 _canairlaunch_3 _caninputrotation_3 _magnettoenemy_3 _airtime_3) (break `/Game/Player/BattleSystem/S_Attack` (`self.GetAttackData` (`self.CurrentAttack`))))
  (bind _returnvalue_5 (`KismetMathLibrary.SelectFloat` _hitboxrange_3 (* _hitboxrange_3 (`self.AerialRangeMultiplier`)) (`|EnumEquality` (`self.GetMovementMode`) "MOVE_Walking")))
  (bind _returnvalue_6 (+ (`Actor.K2_GetActorLocation` _ownercharacter) (* (`Actor.GetActorForwardVector` _ownercharacter) (* _returnvalue_5 0.5))))
  (switch `/Game/Player/BattleSystem/E_HitboxType` (`.HitboxType_44_DFA17E1940B0D2DF6AFD3288B251C4EE` (break `/Game/Player/BattleSystem/S_Attack` (`self.GetAttackData` (`self.CurrentAttack`))))
    (:`NewEnumerator0`
      (bind _outhits (`KismetSystemLibrary.SphereTraceMulti` :`Start` (+ _returnvalue (* _returnvalue_2 50.0)) :`End` (+ _returnvalue (* _returnvalue_2 (`KismetMathLibrary.SelectFloat` _hitboxrange_2 (* _hitboxrange_2 (`self.AerialRangeMultiplier`)) (`|EnumEquality` (`self.GetMovementMode`) "MOVE_Walking")))) :`Radius` 50.0 :`TraceChannel` "TraceTypeQuery4" :`DrawDebugType` "ForDuration" :`DrawTime` 1.0))
      (for _array_element _outhits
        (`KismetArrayLibrary.Array_AddUnique` (`local.GroundedEnemies`) (`.HitActor` (`GameplayStatics.BreakHitResult` _array_element))))
      (`self.DmgHitActors` (`local.GroundedEnemies`) _damage_2 0.0 true _launchforce_2 _canbreakguard_2 _cantrigger2d_2 _canairlaunch_2 _airtime_2 0.0 (`local.HitType`)))
    (:`NewEnumerator2`
      (bind _outhits_2 (`KismetSystemLibrary.SphereTraceMulti` :`Start` (+ _returnvalue_6 (* _returnvalue_3 -35.0)) :`End` (+ _returnvalue_6 (* _returnvalue_3 35.0)) :`Radius` _returnvalue_5 :`TraceChannel` "TraceTypeQuery4" :`DrawDebugType` "ForDuration" :`DrawTime` 1.0))
      (for _array_element_2 _outhits_2
        (`KismetArrayLibrary.Array_AddUnique` (`local.GroundedEnemies`) (`.HitActor` (`GameplayStatics.BreakHitResult` _array_element_2))))
      (`self.DmgHitActors` (`local.GroundedEnemies`) _damage_3 0.0 true _launchforce_3 _canbreakguard_3 _cantrigger2d_3 _canairlaunch_3 _airtime_3 0.0 (`local.HitType`)))
    (:`NewEnumerator1`
      (bind _outhits_3 (`KismetSystemLibrary.SphereTraceMulti` :`Start` _returnvalue_4 :`End` _returnvalue_4 :`Radius` _hitboxrange :`TraceChannel` "TraceTypeQuery4" :`DrawDebugType` "ForDuration" :`DrawTime` 1.0))
      (for _array_element_3 _outhits_3
        (bind (_bblockinghit _binitialoverlap _time _distance _location _impactpoint _normal _impactnormal _physmat _hitactor) (`GameplayStatics.BreakHitResult` _array_element_3))
        (if (<= (`KismetMathLibrary.Abs` (- (`.Z` (`KismetMathLibrary.BreakVector3f` (`Actor.K2_GetActorLocation` _hitactor))) (`.Z` (`KismetMathLibrary.BreakVector3f` _returnvalue_4)))) 210.0)
          (`KismetArrayLibrary.Array_AddUnique` (`local.GroundedEnemies`) _hitactor)))
      (`self.DmgHitActors` (`local.GroundedEnemies`) _damage 0.0 true _launchforce _canbreakguard _cantrigger2d _canairlaunch _airtime 0.0 (`local.HitType`)))))

(fn `ToggleOneShot`
  (bind _output_get (set `self.OneShot` (not (`self.OneShot`))))
  (`KismetSystemLibrary.PrintString` (`KismetStringLibrary.Conv_BoolToString` _output_get)))

(fn `TryNextAttack`
  (if (and (not (`self.IsAttacking`)) (not (`self.IsDash`)))
    (if (`self.LightChargedBuffer`)
      (set `self.CurrentAttack` "NewEnumerator20")
      (set `self.BufferedAttack` "NewEnumerator4")
      (`self.PlayAttackAnimation` "NewEnumerator20")
      (elif (`self.HeavyChargedBuffer`)
        (set `self.CurrentAttack` "NewEnumerator21")
        (set `self.BufferedAttack` "NewEnumerator4")
        (`self.PlayAttackAnimation` "NewEnumerator21")
        (elif (`|EnumInequality` (`self.BufferedAttack`) "NewEnumerator4")
          (`self.PlayAttackAnimation` (`self.BufferedAttack`)))))))