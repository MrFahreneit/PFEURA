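; BP_BGMTrigger is a trigger actor that changes or stops background music.
; It fires shortly after BeginPlay if TriggerOnStart is set, or when a BP_Player or BP_2DPlayer overlaps its box, with a TriggerOnce option.
; PlayType selects a new track, a non-overlapping new track or a stop, with configurable fades.
; Calls go to the BGM manager from GM_gameplay, falling back to a BP_BGMManager actor search under other game modes.
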(event `self.ReceiveBeginPlay`
  (`KismetSystemLibrary.DelayUntilNextTick`)
  (if (`self.TriggerOnStart`)
    (if (`self.TriggerOnce`) :!label _label
      (`/Engine/EditorBlueprintResources/StandardMacros.DoOnce` false
        (:`Completed`
          _)))
    (`self.TriggerBGM`)))

(event `self.Box.OnComponentBeginOverlap`
  (params (OverlappedComponent :type "PrimitiveComponent Object Reference") (OtherActor :type "Actor Object Reference") (OtherComp :type "PrimitiveComponent Object Reference") (OtherBodyIndex :type Integer) (bFromSweep :type Boolean) (SweepResult :type "HitResult Structure (by ref)"))
  (cast `/Game/Player/BP_Player` OtherActor
    (:`then`
      (goto _label))
    (:`CastFailed`
      (cast `/Game/Player/2DPlayer/BP_2DPlayer` OtherActor)
      (goto _label))))

(fn `GetBGMManager`
  (returns (BGMManager :type "/Game/ScoresAndSountrack/BP_BGMManager Object Reference"))
  (bind _asgm_gameplay (cast `/Game/InstanceAndGamemode/GM_gameplay` (`GameplayStatics.GetGameMode`))
    (:`then`
      (return (`/Game/InstanceAndGamemode/GM_gameplay.BGMManager` _asgm_gameplay)))
    (:`CastFailed`
      (bind _returnvalue (`GameplayStatics.GetActorOfClass` "/Game/ScoresAndSountrack/BP_BGMManager.BP_BGMManager_C"))
      (return _returnvalue))))

(fn `TriggerBGM`
  (bind _bgmmanager (`self.GetBGMManager`))
  (if (`KismetSystemLibrary.IsValid` _bgmmanager)
    (switch `/Game/ScoresAndSountrack/E_BGMPlayType` (`self.PlayType`)
      (:`NewEnumerator1`
        (`/Game/ScoresAndSountrack/BP_BGMManager.PlayNewBGM` _bgmmanager (`self.FadeOutDuration`) (`self.BGMToPlay`) (`self.FadeInDuration`)))
      (:`NewEnumerator2`
        (`/Game/ScoresAndSountrack/BP_BGMManager.PlayNewBGMNoOverlap` _bgmmanager (`self.FadeOutDuration`) (`self.BGMToPlay`) (`self.FadeInDuration`) (`self.NewFadeInDelay`)))
      (:`NewEnumerator3`
        (`/Game/ScoresAndSountrack/BP_BGMManager.StopBGM` _bgmmanager (`self.FadeOutDuration`))))))

(fn `UserConstructionScript`)