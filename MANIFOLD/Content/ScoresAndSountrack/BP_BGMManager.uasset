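; BP_BGMManager manages background music, starting and stopping tracks with fade-in and fade-out.
; StopBGM hands the current audio component to an old slot and fades it out; new tracks spawn as 2D sounds, either immediately for a crossfade or after a delay to avoid overlap.
; Tick polls timestamps to destroy the faded component and launch queued tracks, with -1 marking an empty queue.
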(event `self.ReceiveTick`
  (params (DeltaSeconds :type "Float (single-precision)"))
  (`|ExecutionSequence`
    (:`then_0`
      (`self.TryDestroyMusicComponent`))
    (:`then_1`
      (`self.TryPlayNewBGM`))))

(fn `PlayBGM`
  (params (BGMToPlay :type "SoundCue Object Reference") (FadeInDuration :type "Float (single-precision)"))
  (bind _returnvalue (`GameplayStatics.SpawnSound2D` BGMToPlay 1.0 1.0 0.0 null))
  (bind _output_get (set `self.CurrentBGM` _returnvalue))
  (`AudioComponent.FadeIn` _output_get FadeInDuration 1.0 0.0 "Linear"))

(fn `PlayNewBGM`
  (params (FadeOutDuration :type "Float (single-precision)") (BGMToPlay :type "SoundCue Object Reference") (FadeInDuration :type "Float (single-precision)"))
  (`self.StopBGM` FadeOutDuration)
  (`self.PlayBGM` BGMToPlay FadeInDuration))

(fn `PlayNewBGMNoOverlap`
  (params (FadeOutDuration :type "Float (single-precision)") (BGMToPlay :type "SoundCue Object Reference") (FadeInDuration :type "Float (single-precision)") (NewFadeInDelay :type "Float (double-precision)"))
  (`self.StopBGM` FadeOutDuration)
  (set `self.NewFadeInDelay` (+ NewFadeInDelay (`GameplayStatics.GetTimeSeconds`)))
  (set `self.NewBGMFadeIn` FadeInDuration)
  (set `self.NewCueToPlay` BGMToPlay))

(fn `StopBGM`
  (params (FadeOutDuration :type "Float (single-precision)"))
  (bind _currentbgm (`self.CurrentBGM`))
  (`/Engine/EditorBlueprintResources/StandardMacros.IsValid` _currentbgm
    (:`Is Valid`
      (set `self.OldBGM` _currentbgm)
      (set `self.CurrentBGM` null)
      (`AudioComponent.FadeOut` (`self.OldBGM`) FadeOutDuration 0.0 "Linear")
      (set `self.DestroyTimerStart` (+ (+ FadeOutDuration (`GameplayStatics.GetTimeSeconds`)) 0.1)))))

(fn `TryDestroyMusicComponent`
  (bind _oldbgm (`self.OldBGM`))
  (if (>= (`GameplayStatics.GetTimeSeconds`) (`self.DestroyTimerStart`))
    (`/Engine/EditorBlueprintResources/StandardMacros.IsValid` _oldbgm
      (:`Is Valid`
        (`ActorComponent.K2_DestroyComponent` _oldbgm)))))

(fn `TryPlayNewBGM`
  (bind _currentbgm (`self.CurrentBGM`))
  (if (!= (`self.NewFadeInDelay`) -1.0)
    (if (>= (`GameplayStatics.GetTimeSeconds`) (`self.NewFadeInDelay`))
      (`/Engine/EditorBlueprintResources/StandardMacros.IsValid` _currentbgm
        (:`Is Valid`
          (`ActorComponent.K2_DestroyComponent` _currentbgm))
        (:`Is Not Valid`
          _))
      (`self.PlayBGM` (`self.NewCueToPlay`) (`self.NewBGMFadeIn`))
      (set `self.NewFadeInDelay` -1.0))))

(fn `UserConstructionScript`)