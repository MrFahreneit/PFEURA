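; Gameplay GameMode that sets up the level on BeginPlay and handles checkpoint respawns for the player.
; BeginPlay caps FPS, plays a fade from black, finds the BGM manager, caches GameInstance and player, and seeds an unset checkpoint from the player's transform.
; RespawnPlayer runs a DoOnce-gated, delay-timed sequence: exit 2D, lock input, grant invincibility, detach camera, teleport to the GameInstance checkpoint behind a transition widget, then restore everything.
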(event `self.ReceiveBeginPlay`
  (bind (_checkpointtransform_location _checkpointtransform_rotation) (`KismetMathLibrary.BreakTransform` (`/Game/InstanceAndGamemode/GI_MasterInst.CheckPointTransform` (`self.As GI Master Inst`))))
  (`KismetSystemLibrary.ExecuteConsoleCommand` "t.maxfps 60" null)
  (bind _returnvalue (`|CreateWidget` "/Game/UI/Widgets/W_TransitionBlack.W_TransitionBlack_C"))
  (`UserWidget.AddToViewport` _returnvalue 0)
  (`UserWidget.PlayAnimation` _returnvalue (`/Game/UI/Widgets/W_TransitionBlack.Transition` _returnvalue) 0.0 1 "Reverse" 1.0 false)
  (`self.initializeBGMManager`)
  (bind _asgi_master_inst (cast `/Game/InstanceAndGamemode/GI_MasterInst` (`GameplayStatics.GetGameInstance`)))
  (set `self.As GI Master Inst` _asgi_master_inst)
  (bind _asbp_player (cast `/Game/Player/BP_Player` (`GameplayStatics.GetPlayerCharacter` 0)))
  (bind _output_get (set `self.As BP Player` _asbp_player))
  (if (and (== _checkpointtransform_location (0.0 0.0 0.0) :`ErrorTolerance` 0.1) (== _checkpointtransform_rotation (struct) :`ErrorTolerance` 0.1))
    (set `/Game/InstanceAndGamemode/GI_MasterInst.CheckPointTransform` (`self.GetTransform` _output_get) (`self.As GI Master Inst`))))

(event `RespawnPlayer`
  (bind _returnvalue (`GameplayStatics.GetPlayerCharacter` 0))
  (bind _2dplayer (`/Game/Player/BP_Player.2DPlayer` (`self.As BP Player`)))
  (bind (_checkpointtransform_location _checkpointtransform_rotation) (`KismetMathLibrary.BreakTransform` (`/Game/InstanceAndGamemode/GI_MasterInst.CheckPointTransform` (`self.As GI Master Inst`))))
  (`/Engine/EditorBlueprintResources/StandardMacros.DoOnce` false :!label _label
    (:`Completed`
      (if (`KismetSystemLibrary.IsValid` _2dplayer)
        (`/Game/Player/2DPlayer/BP_2DPlayer.Exit2D` _2dplayer))
      (`self.DisableInput` _returnvalue (`GameplayStatics.GetPlayerController` 0))
      (`KismetSystemLibrary.Delay` 0.2) ; Let 2DExit Anim play
      (bind _asbp_player (cast `/Game/Player/BP_Player` _returnvalue)
        (:`then`
          (`/Game/Player/BP_Player.ForceStopRun` _asbp_player)
          (set `/Game/Player/BP_Player.Invicibility` true _asbp_player))
        (:`CastFailed`
          _))
      (`/Game/Player/BP_Player.DetachCamera` (`self.As BP Player`))
      (`KismetSystemLibrary.Delay` 0.8)
      (`/Engine/EditorBlueprintResources/StandardMacros.IsValid` (`self.TransitionWidget`)
        (:`Is Valid`
          _)
        (:`Is Not Valid`
          (bind _returnvalue_2 (`|CreateWidget` "/Game/UI/Widgets/W_Transition.W_Transition_C"))
          (bind _output_get (set `self.TransitionWidget` _returnvalue_2))
          (`UserWidget.AddToViewport` _output_get 9999)))
      (`UserWidget.PlayAnimationForward` (`self.TransitionWidget`) (`/Game/UI/Widgets/W_Transition.Transition` (`self.TransitionWidget`)) 1.0 false)
      (`KismetSystemLibrary.Delay` 1.0) ; Wait animation end before TP
      (`self.K2_SetActorTransform` (`self.As BP Player`) (`KismetMathLibrary.MakeTransform` _checkpointtransform_location _checkpointtransform_rotation) false true)
      (`Controller.SetControlRotation` (`GameplayStatics.GetPlayerController` 0) (`KismetMathLibrary.MakeRotator` 0.0 -45.0 (.yaw _checkpointtransform_rotation)))
      (`/Game/Player/BP_Player.ReAttachCamera` (`self.As BP Player`))
      (`KismetSystemLibrary.Delay` 0.5) ; Wait before ending transition
      (`UserWidget.PlayAnimationReverse` (`self.TransitionWidget`) (`/Game/UI/Widgets/W_Transition.Transition` (`self.TransitionWidget`)) 1.0 false)
      (`KismetSystemLibrary.Delay` 0.3)
      (`self.EnableInput` (`GameplayStatics.GetPlayerCharacter` 0) (`GameplayStatics.GetPlayerController` 0))
      (`self.ResetRespawnPlayer`)
      (`KismetSystemLibrary.Delay` 1.0)
      (set `/Game/Player/BP_Player.Invicibility` false (`self.As BP Player`)))))

(event `ResetRespawnPlayer`
  (goto _label :!via `Reset`))

(fn `initializeBGMManager`
  (bind _outactors (`GameplayStatics.GetAllActorsOfClass` "/Game/ScoresAndSountrack/BP_BGMManager.BP_BGMManager_C"))
  (for (_array_element _array_index) _outactors
    (if (> _array_index 0)
      (`KismetSystemLibrary.PrintString` "MULTIPLE BGM MANAGER DETECTED" true false (struct :`R` 1.0 :`G` 0.026519 :`A` 1.0))
      (else
        (set `self.BGMManager` _array_element)
        (`KismetSystemLibrary.PrintString` "BGM MANAGER FOUND" true false (struct :`G` 1.0 :`B` 0.086479 :`A` 1.0))))))

(fn `StartHitStopEndHitStop`)

(fn `UserConstructionScript`)