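; Arena game mode that tracks the player's score during fights in a BP_FightRoom and stores the arena ID.
; BeginPlay caches the fight room, and EntityKilled increments Score only for entities carrying an AC_WaveEntity component.
; On player death it pauses everything else in the room, ends the fight and shows W_ArenaScore with the arena ID, score and highscore.
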(event `self.ReceiveBeginPlay`
  (`parent.ReceiveBeginPlay`)
  (bind _returnvalue (`GameplayStatics.GetActorOfClass` "/Game/Interactif/AI/BP_FightRoom.BP_FightRoom_C"))
  (set `self.FightRoom` _returnvalue))

(event `PlayerDeath`
  (bind _fightroom (`self.FightRoom`))
  (`/Game/Interactif/AI/BP_FightRoom.PauseAllOther` _fightroom null)
  (`/Game/Interactif/AI/BP_FightRoom.FightFinished` _fightroom)
  (bind _returnvalue (`|CreateWidget` "/Game/UI/Widgets/Arena/W_ArenaScore.W_ArenaScore_C" null (`self.ArenaID`) (`self.Score`) (`self.Highscore`)))
  (`UserWidget.AddToViewport` _returnvalue 0))

(fn `EntityKilled`
  (params (Entity :type "Actor Object Reference"))
  (if (`KismetSystemLibrary.IsValid` (`self.GetComponentByClass` Entity "/Game/Interactif/AI/WaveSystem/AC_WaveEntity.AC_WaveEntity_C"))
    (`/Engine/EditorBlueprintResources/StandardMacros.IncrementInt` (`self.Score`))))

(fn `GetArenaID`
  (returns (ArenaID :type Integer))
  (return (`self.ArenaID`)))

(fn `SetArenaID`
  (params (ArenaID :type Integer))
  (set `self.ArenaID` ArenaID))

(fn `UserConstructionScript`
  (`parent.UserConstructionScript`))