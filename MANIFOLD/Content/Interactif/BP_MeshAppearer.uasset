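; BP_MeshAppearer is an interactive actor that keeps a configurable mesh hidden and non-colliding until an interaction starts.
; The construction script applies the Mesh variable to the static mesh, and BeginPlay hides it and disables collision on it and on the Cube of its BP_2DBlock child actor.
; STARTINTERACTION reveals the mesh and sets both components to QueryAndProbe collision, with no logic to hide it again.
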(event `self.ReceiveBeginPlay`
  (`SceneComponent.SetVisibility` (`self.StaticMesh`) false false)
  (bind _asbp_2dblock (cast `/Game/Interactif/2D/BP_2DBlock` (`ChildActorComponent.ChildActor` (`self.ChildActor`))))
  (`PrimitiveComponent.SetCollisionEnabled` (`/Game/Interactif/2D/BP_2DBlock.Cube` _asbp_2dblock) "NoCollision")
  (`PrimitiveComponent.SetCollisionEnabled` (`self.StaticMesh`) "NoCollision"))

(event `/Game/Interactif/BPI_Interactible.START_INTERACTION`
  (bind _staticmesh (`self.StaticMesh`))
  (`SceneComponent.SetVisibility` _staticmesh true false)
  (bind _asbp_2dblock (cast `/Game/Interactif/2D/BP_2DBlock` (`ChildActorComponent.ChildActor` (`self.ChildActor`))))
  (`PrimitiveComponent.SetCollisionEnabled` _staticmesh "QueryAndProbe")
  (`PrimitiveComponent.SetCollisionEnabled` (`/Game/Interactif/2D/BP_2DBlock.Cube` _asbp_2dblock) "QueryAndProbe"))

(fn `UserConstructionScript`
  (`StaticMeshComponent.SetStaticMesh` (`self.StaticMesh`) (`self.mesh`)))