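; Enemy ranged laser attack that, despite its name, is a timed beam with no movement or collision.
; A Niagara targeting beam tracks the player on Tick, then after a delay a firing beam spawns, unless the player is in a combo.
; The shot damages the player automatically unless tracking has broken, either by the player's dash event or by running after a short grace period, which freezes the beam's end.
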(event `self.ReceiveBeginPlay`
  (bind _as_bp_player (`self.As BP Player`))
  (bind _asbp_player (cast `/Game/Player/BP_Player` (`GameplayStatics.GetPlayerCharacter` 0)))
  (bind _output_get (set `self.As BP Player` _asbp_player))
  (add `/Game/Player/BP_Player.HasDashed` _output_get (delegate `StopFollowing`))
  (`GameplayStatics.PlaySoundAtLocation` "/Game/SFX/Cues/RangedCall_Cue.RangedCall_Cue" (`self.K2_GetActorLocation`) (struct) 1.0 1.0 0.0 null null null null)
  (`self.SpawnParticle`)
  (`|ExecutionSequence`
    (:`then_0`
      (`KismetSystemLibrary.K2_SetTimer` null "SpawnParticle" 4.0 true)
      (bind _returnvalue (`NiagaraFunctionLibrary.SpawnSystemAttached` "/Game/GA/NiagaraSystems/NS_ProjectileEnemyLaserCible.NS_ProjectileEnemyLaserCible" (`self.Scene`) "None" (`self.K2_GetActorLocation`) (struct) "KeepWorldPosition"))
      (bind _output_get_2 (set `self.laserSpawned` _returnvalue))
      (`FXSystemComponent.SetVectorParameter` _output_get_2 "BeamEnd" (`self.K2_GetActorLocation` (`GameplayStatics.GetPlayerCharacter` 0)))
      (`KismetSystemLibrary.Delay` 2.7)
      (if (not (`/Game/Player/BP_Player.isInCombo` (`self.As BP Player`)))
        (bind _returnvalue_2 (`NiagaraFunctionLibrary.SpawnSystemAttached` "/Game/GA/NiagaraSystems/NS_ProjectileEnemyLaserEM.NS_ProjectileEnemyLaserEM" (`self.Scene`) "None" (`self.K2_GetActorLocation`) (struct) "KeepWorldPosition"))
        (set `self.Cible` _returnvalue_2)
        (`FXSystemComponent.SetVectorParameter` _returnvalue_2 "BeamEnd" (select `bool` (`self.stopFollow`) :`false` (`self.K2_GetActorLocation` (`GameplayStatics.GetPlayerCharacter` 0)) :`true` (+ (`self.K2_GetActorLocation`) (* (`KismetMathLibrary.Normal` (- (`self.BeamEnd`) (`self.K2_GetActorLocation`))) 10000.0))))
        (`GameplayStatics.SpawnSoundAtLocation` "/Game/SFX/Cues/RangedShot_Cue.RangedShot_Cue" (`self.K2_GetActorLocation`) (struct) 1.0 1.0 0.0 null null)
        (if (not (`self.stopFollow`))
          (`/Game/Player/BP_Player.LoseHealth` _as_bp_player (`self.Damages`))
          (`NiagaraFunctionLibrary.SpawnSystemAtLocation` "/Game/GA/NiagaraSystems/NS_HitLaser.NS_HitLaser" (`self.K2_GetActorLocation` _as_bp_player)))))
    (:`then_1`
      (`KismetSystemLibrary.Delay` 0.75)
      (goto _label :!via `Open`))))

(event `StopFollowing`
  (set `self.stopFollow` true))

(event `SpawnParticle`)

(event `self.ReceiveTick`
  (params (DeltaSeconds :type "Float (single-precision)"))
  (bind _cible (`self.Cible`))
  (bind _laserspawned (`self.laserSpawned`))
  (bind _beamend (`self.BeamEnd`))
  (`|ExecutionSequence`
    (:`then_0`
      (`/Engine/EditorBlueprintResources/StandardMacros.Gate` true :!label _label
        (:`Exit`
          (if (`/Game/Player/BP_Player.IsRunning` (`self.As BP Player`))
            (set `self.stopFollow` true)))))
    (:`then_1`
      (if (`self.stopFollow`)
        (`/Engine/EditorBlueprintResources/StandardMacros.DoOnce` false
          (:`Completed`
            (bind _output_get (set `self.BeamEnd` (`self.GetBeamEndLoc`)))
            (`FXSystemComponent.SetVectorParameter` (`self.laserSpawned`) "BeamEnd" _output_get)))
        (else
          (set `self.BeamEnd` (`self.K2_GetActorLocation` (`GameplayStatics.GetPlayerCharacter` 0)))
          (`/Engine/EditorBlueprintResources/StandardMacros.IsValid` _cible
            (:`Is Valid`
              (`FXSystemComponent.SetVectorParameter` _cible "BeamEnd" _beamend))
            (:`Is Not Valid`
              _))
          (`/Engine/EditorBlueprintResources/StandardMacros.IsValid` _laserspawned
            (:`Is Valid`
              (`FXSystemComponent.SetVectorParameter` _laserspawned "BeamEnd" (select `bool` (`self.stopFollow`) :`false` _beamend :`true` (+ (`self.K2_GetActorLocation`) (* (`KismetMathLibrary.Normal` (- (`self.BeamEnd`) (`self.K2_GetActorLocation`))) 10000.0)))))))))))

(fn `GetBeamEndLoc`
  (returns (ReturnValue :type "Vector Structure"))
  (return (* (- (`self.K2_GetActorLocation` (`GameplayStatics.GetPlayerCharacter` 0)) (`self.K2_GetActorLocation`)) 1000.0)))

(fn `UserConstructionScript`)