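; AC_AIDrop is an actor component that makes its AI owner drop health and experience orbs.
; SpawnDrop calls SpawnOrb once for each configured health orb and experience orb.
; SpawnOrb spawns a BP_Coin at a random offset around and above the owner's location, flagged as health or experience and carrying the configured HP and Exp values.
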(fn `SpawnDrop`
  (for _ (range 1 (+ (`self.NHealthOrb`) 1))
    (`self.SpawnOrb` true))
  (for _ (range 1 (+ (`self.NExpOrb`) 1))
    (`self.SpawnOrb` false)))

(fn `SpawnOrb`
  (params (IsHealth :type Boolean))
  (bind (_x _y _z) (`KismetMathLibrary.BreakVector3f` (`Actor.K2_GetActorLocation` (`self.GetOwner`))))
  (`|SpawnActorFromClass` "/Game/Interactif/Orbs/BP_Coin.BP_Coin_C" (`KismetMathLibrary.MakeTransform` (`KismetMathLibrary.MakeVector` (+ _x (`KismetMathLibrary.RandomFloatInRange` -300.0 300.0)) (+ _y (`KismetMathLibrary.RandomFloatInRange` -300.0 300.0)) (+ _z (`KismetMathLibrary.RandomFloatInRange` 80.0 300.0)))) "Undefined" "OverrideRootScale" null true IsHealth (`self.HPOrbValue`) (`self.ExpOrbValue`) null))