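; AC_Hitframe is an actor component that provides a hit-freeze effect by briefly stopping time.
; StartHitFrame sets either global time dilation or the owner's CustomTimeDilation to zero, depending on its Global flag.
; It clears any pending timer and schedules EndHitFrame after the given time, which restores the dilation selected by the stored flag to normal.
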(event `self.ReceiveBeginPlay`
  (set `self.Owner` (`self.GetOwner`)))

(fn `EndHitFrame`
  (if (`self.Global?`)
    (`GameplayStatics.SetGlobalTimeDilation` 1.0)
    (else
      (set `Actor.CustomTimeDilation` 1.0 (`self.Owner`)))))

(fn `StartHitFrame`
  (params (Time :type "Float (single-precision)") (`global?` :type Boolean))
  (`KismetSystemLibrary.K2_ClearAndInvalidateTimerHandle` (`self.HitFrameTimer`))
  (bind _output_get (set `self.Global?` `global?`))
  (if _output_get
    (`GameplayStatics.SetGlobalTimeDilation` 0.0)
    (else
      (set `Actor.CustomTimeDilation` 0.0 (`self.Owner`))))
  (bind _returnvalue (`KismetSystemLibrary.K2_SetTimer` null "EndHitFrame" Time))
  (set `self.HitFrameTimer` _returnvalue))