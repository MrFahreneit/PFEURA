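; BP_CineEnterBoss is a one-shot trigger box that launches the boss entrance cinematic when the player overlaps it.
; It hides the HUD, activates ACInteractible movement toward MovePoint, then after a short delay starts the FightRoomBoss fight and the player's entrance cinematic.
; Timed delays sequence the music, fading out the BGM and later starting the boss track.
; An older camera blend and follow path remains in the graph but never runs.
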(event `Start`
  (`/Engine/EditorBlueprintResources/StandardMacros.DoOnce` false
    (:`Completed`
      (bind _asbp_player (cast `/Game/Player/BP_Player` (`GameplayStatics.GetPlayerCharacter` 0)))
      (`/Game/UI/Widgets/HUD/W_HUD.Hide UI` (`/Game/Player/BP_Player.HUD_Widget` _asbp_player))
      (`/Game/Interactif/AC_Interactible.ActivateMovement` (`self.AC_Interactible`))
      (`KismetSystemLibrary.Delay` 0.5)
      (`/Game/Interactif/AI/BP_FightRoom.StartFight` (`self.FightRoomBoss`))
      (bind _asbp_player_2 (cast `/Game/Player/BP_Player` (`GameplayStatics.GetPlayerCharacter` 0)))
      (`/Game/Player/BP_Player.StartBossEnterCine` _asbp_player_2)
      (bind _asgm_gameplay (cast `/Game/Player/GM_gameplay` (`GameplayStatics.GetGameMode`)))
      (`/Game/ScoresAndSountrack/BP_BGMManager.StopBGM` (`/Game/Player/GM_gameplay.BGMManager` _asgm_gameplay) 2.0)
      (`KismetSystemLibrary.Delay` 18.0)
      (bind _asgm_gameplay_2 (cast `/Game/Player/GM_gameplay` (`GameplayStatics.GetGameMode`)))
      (`/Game/ScoresAndSountrack/BP_BGMManager.PlayNewBGM` (`/Game/Player/GM_gameplay.BGMManager` _asgm_gameplay_2) 0.0 "/Game/ScoresAndSountrack/5DAberration_Cue.5DAberration_Cue" 0.0))))

(event `self.ReceiveTick`
  (params (DeltaSeconds :type "Float (single-precision)")))

(event `self.ReceiveBeginPlay`
  ;[1 1 1] ToCopy
  (set `/Game/Interactif/AC_Interactible.ObjectifMovement` (`self.MovePoint`) (`self.AC_Interactible`)))

(event `self.Box.OnComponentBeginOverlap`
  (params (OverlappedComponent :type "PrimitiveComponent Object Reference") (OtherActor :type "Actor Object Reference") (OtherComp :type "PrimitiveComponent Object Reference") (OtherBodyIndex :type Integer) (bFromSweep :type Boolean) (SweepResult :type "HitResult Structure (by ref)"))
  (cast `/Game/Player/BP_Player` OtherActor)
  (`self.Start`))

(fn `UserConstructionScript`)