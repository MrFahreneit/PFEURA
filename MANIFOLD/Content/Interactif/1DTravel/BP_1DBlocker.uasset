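; BP_1DBlocker is a quick-time-event obstacle in 1D travel, typed as Dash, LightAttack or HeavyAttack, which sets its button icon and color.
; A camera-facing scene component updates each tick, while player overlap pops the prompt and registers the blocker as the controller's current one.
; Passe plays effects, hides the prompt and timeline-lerps the player to TPPoint.
; BP_Boss1D overlapping the second box triggers only effects and sound.
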(event `self.ReceiveBeginPlay`
  (`Image.SetBrushFromTexture` (`/Game/UI/Widgets/W_Input.Image_21` (cast `/Game/UI/Widgets/W_Input` (`WidgetComponent.GetWidget` (`self.Input`)) :!pure true)) (select `/Game/Interactif/1DTravel/Enum_1DQTE` (`self.currentQTE`) :`NewEnumerator0` "/Game/UI/Assets/Inputs/64x64/B.B" :`NewEnumerator1` "/Game/UI/Assets/Inputs/64x64/X.X" :`NewEnumerator2` "/Game/UI/Assets/Inputs/64x64/Y.Y" :!type "Texture2D Object Reference") false)
  (bind _returnvalue (`PrimitiveComponent.CreateDynamicMaterialInstance` (`self.Plane`) 0 "/Game/GA/Materials/Other/M_MaskedUnlit.M_MaskedUnlit" "None"))
  (bind _output_get (set `self.ColorMat` _returnvalue))
  (`MaterialInstanceDynamic.SetVectorParameterValue` _output_get "Color" (select `/Game/Interactif/1DTravel/Enum_1DQTE` (`self.currentQTE`) :`NewEnumerator0` (struct :`R` 1.0 :`B` 0.017682 :`A` 1.0) :`NewEnumerator1` (struct :`G` 0.237913 :`B` 1.0 :`A` 1.0) :`NewEnumerator2` (struct :`R` 1.0 :`G` 0.814225 :`A` 1.0) :!type "LinearColor Structure")))

(event `self.ReceiveTick`
  (params (DeltaSeconds :type "Float (single-precision)"))
  (bind _scene (`self.Scene`))
  (`SceneComponent.K2_SetWorldRotation` _scene (`KismetMathLibrary.FindLookAtRotation` (`SceneComponent.K2_GetComponentLocation` _scene) (`SceneComponent.K2_GetComponentLocation` (`PlayerCameraManager.TransformComponent` (`GameplayStatics.GetPlayerCameraManager` 0)))) false true))

(event `Passe`
  (params (Player1D :type "/Game/Interactif/1DTravel/BP_1DController Object Reference"))
  (bind _asw_input (cast `/Game/UI/Widgets/W_Input` (`WidgetComponent.GetWidget` (`self.Input`)) :!pure true))
  (set `self.isPass?` true)
  (`NiagaraFunctionLibrary.SpawnSystemAtLocation` "/Game/GA/NiagaraSystems/NS_PunchNormal.NS_PunchNormal" (`self.K2_GetActorLocation`) (struct) (0.3 0.3 0.3))
  (`TimelineComponent.SetPlayRate` (`self.MovePoint`) (/ 1.0 0.2))
  (`GameplayStatics.PlaySound2D` "/Game/SFX/Cues/1D_BlockerPass_Cue.1D_BlockerPass_Cue" 1.0 1.0 0.0 null null)
  (set `self.PointA` (`self.K2_GetActorLocation` Player1D))
  (`UserWidget.PlayAnimation` _asw_input (`/Game/UI/Widgets/W_Input.Pop` _asw_input) 0.0 1 "Reverse" 1.0 false)
  (bind (_direction _alpha) (`Timeline|MovePoint` :!via `PlayFromStart`)
    (:`Update`
      (`self.K2_SetActorLocation` Player1D (`KismetMathLibrary.VLerp` (`self.PointA`) (`SceneComponent.K2_GetComponentLocation` (`self.TPPoint`)) _alpha) false false))))

(event `self.Box.OnComponentBeginOverlap`
  (params (OverlappedComponent :type "PrimitiveComponent Object Reference") (OtherActor :type "Actor Object Reference") (OtherComp :type "PrimitiveComponent Object Reference") (OtherBodyIndex :type Integer) (bFromSweep :type Boolean) (SweepResult :type "HitResult Structure (by ref)"))
  (bind _asw_input (cast `/Game/UI/Widgets/W_Input` (`WidgetComponent.GetWidget` (`self.Input`)) :!pure true))
  (bind _asbp_1dcontroller (cast `/Game/Interactif/1DTravel/BP_1DController` OtherActor))
  (if (not (`self.isPass?`))
    (`UserWidget.PlayAnimation` _asw_input (`/Game/UI/Widgets/W_Input.Pop` _asw_input) 0.0 1 "Forward" 1.0 false)
    (set `/Game/Interactif/1DTravel/BP_1DController.current1DBlocker` self _asbp_1dcontroller)))

(event `self.Box1.OnComponentBeginOverlap`
  (params (OverlappedComponent :type "PrimitiveComponent Object Reference") (OtherActor :type "Actor Object Reference") (OtherComp :type "PrimitiveComponent Object Reference") (OtherBodyIndex :type Integer) (bFromSweep :type Boolean) (SweepResult :type "HitResult Structure (by ref)"))
  (cast `/Game/Interactif/1DTravel/BP_Boss1D` OtherActor)
  (`NiagaraFunctionLibrary.SpawnSystemAtLocation` "/Game/GA/NiagaraSystems/NS_PunchNormal.NS_PunchNormal" (`self.K2_GetActorLocation`) (struct) (0.3 0.3 0.3))
  (`GameplayStatics.PlaySound2D` "/Game/SFX/Cues/1D_BlockerPassBoss_Cue.1D_BlockerPassBoss_Cue" 1.0 1.0 0.0 null null))

(event `self.Box.OnComponentEndOverlap`
  (params (OverlappedComponent :type "PrimitiveComponent Object Reference") (OtherActor :type "Actor Object Reference") (OtherComp :type "PrimitiveComponent Object Reference") (OtherBodyIndex :type Integer))
  (bind _asbp_1dcontroller (cast `/Game/Interactif/1DTravel/BP_1DController` OtherActor))
  (if (== _asbp_1dcontroller self)
    (set `/Game/Interactif/1DTravel/BP_1DController.current1DBlocker` null _asbp_1dcontroller)))

(fn `UserConstructionScript`)