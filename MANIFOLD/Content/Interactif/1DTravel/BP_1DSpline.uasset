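; Spline path actor that periodically spawns BP_1DPassenger actors, passing each itself as the line and a travel speed.
; If CanSpawn is set, a self-recalling Spawner event runs on a randomized delay, skipping spawns during fights and tracking passengers in BouleList.
; ChangeState sets the fight flag and, with ReverseOnFight, forwards it to tracked passengers.
; The construction script tiles spline meshes in sections sized by actor X scale, with clamped tangents.
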(event `self.ReceiveBeginPlay`
  (if (`self.canSpawn?`)
    (`self.Spawner`)))

(event `ChangeState`
  (params (Fight :type Boolean))
  (bind _output_get (set `self.isInFight` Fight))
  (if (`self.reverseOnFight?`)
    (if _output_get
      (for _array_element (`self.BouleList`)
        (`/Engine/EditorBlueprintResources/StandardMacros.IsValid` _array_element
          (:`Is Valid`
            (`/Game/Interactif/1DTravel/BP_1DPassenger.ChangeState` _array_element true))))
      (else
        (for _array_element_2 (`self.BouleList`)
          (`/Engine/EditorBlueprintResources/StandardMacros.IsValid` _array_element_2
            (:`Is Valid`
              (`/Game/Interactif/1DTravel/BP_1DPassenger.ChangeState` _array_element_2 false))))))))

(event `Spawner`
  (if (not (`self.isInFight`))
    (bind _returnvalue (`|SpawnActorFromClass` "/Game/Interactif/1DTravel/BP_1DPassenger.BP_1DPassenger_C" (`KismetMathLibrary.MakeTransform` (`self.K2_GetActorLocation`)) "Undefined" "OverrideRootScale" null self (`self.SpeedPassenger`) null))
    (`KismetArrayLibrary.Array_AddUnique` (`self.BouleList`) _returnvalue))
  (`KismetSystemLibrary.Delay` (`KismetMathLibrary.RandomFloatInRange` (- (`self.TimeSpawn`) (* (`self.TimeSpawn`) (`self.VariationSpawn`))) (+ (* (`self.TimeSpawn`) (`self.VariationSpawn`)) (`self.TimeSpawn`))))
  (`self.Spawner`))

(fn `UserConstructionScript`
  (bind _returnvalue_x (`KismetMathLibrary.BreakVector` (`self.GetActorScale3D`)))
  (bind _spline (`self.Spline`))
  (bind _spline_2 (`self.Spline`))
  (bind _sectionlenght (`self.SectionLenght`))
  (set `self.SectionLenght` (* _returnvalue_x 100.0))
  (for _index (range (`KismetMathLibrary.FTrunc` (/ (`SplineComponent.GetSplineLength` (`self.Spline`)) (`self.SectionLenght`))))
    (bind _returnvalue (`AddComponent|NODE_AddSplineMeshComponent-0`))
    (`SplineMeshComponent.SetForwardAxis` _returnvalue "X" true)
    (bind _returnvalue_2 (* _index _sectionlenght))
    (bind _returnvalue_3 (* (+ _index 1) _sectionlenght))
    (`SplineMeshComponent.SetStartAndEnd` _returnvalue (`SplineComponent.GetLocationAtDistanceAlongSpline` _spline_2 _returnvalue_2 "Local") (`KismetMathLibrary.ClampVectorSize` (`SplineComponent.GetTangentAtDistanceAlongSpline` _spline_2 _returnvalue_2 "Local") 0.0 (`self.SectionLenght`)) (`SplineComponent.GetLocationAtDistanceAlongSpline` _spline _returnvalue_3 "Local") (`KismetMathLibrary.ClampVectorSize` (`SplineComponent.GetTangentAtDistanceAlongSpline` _spline _returnvalue_3 "Local") 0.0 (`self.SectionLenght`)) true)))