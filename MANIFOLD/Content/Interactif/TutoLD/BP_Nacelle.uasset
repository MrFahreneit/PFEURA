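; BP_Nacelle is a moving actor that travels point to point along a referenced spline, started on BeginPlay by a flag or once through StartMove.
; Each leg begins at the spline point nearest the actor and targets the next index, wrapping to the first after the last.
; A timeline lerps location in a straight line, with play rate set from Speed over segment distance.
; After a short pause, the next leg repeats the search.
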(event `self.ReceiveBeginPlay`
  (if (`self.shouldStartOnPlay`)
    (`self.FollowSpline`)))

(event `FollowSpline`
  (bind _pointtostartindex (`self.pointToStartIndex`))
  (bind _spline (`/Game/Interactif/TutoLD/BP_SplineToFollow.Spline` (`self.splineToFollow`)))
  (bind _returnvalue (`SplineComponent.GetLocationAtSplinePoint` (`/Game/Interactif/TutoLD/BP_SplineToFollow.Spline` (`self.splineToFollow`)) (`self.pointToGoIndex`) "World"))
  (bind _returnvalue_2 (`SplineComponent.GetLocationAtSplinePoint` (`/Game/Interactif/TutoLD/BP_SplineToFollow.Spline` (`self.splineToFollow`)) (`self.pointToStartIndex`) "World"))
  (bind _returnvalue_3 (- (`SplineComponent.GetNumberOfSplinePoints` _spline) 1))
  (`self.splineToFollow`
    (:`then`
      (set `self.closestDistance` 99999999999.0)
      (for _index (range (+ _returnvalue_3 1))
        (bind _returnvalue_4 (`KismetMathLibrary.Vector_Distance` (`self.K2_GetActorLocation`) (`SplineComponent.GetLocationAtSplinePoint` _spline _index "World")))
        (if (< _returnvalue_4 (`self.closestDistance`))
          (set `self.closestDistance` _returnvalue_4)
          (set `self.pointToStartIndex` _index)))
      (set `self.pointToGoIndex` (`KismetMathLibrary.SelectInt` 0 (+ _pointtostartindex 1) (== _pointtostartindex _returnvalue_3)))
      (`TimelineComponent.SetPlayRate` (`self.Timeline_FollowSpline`) (/ (`self.speed`) (`KismetMathLibrary.Vector_Distance` _returnvalue_2 _returnvalue)))
      (bind (_direction _track) (`Timeline|Timeline_FollowSpline` :!via `PlayFromStart`)
        (:`Update`
          (`self.K2_SetActorLocation` (`KismetMathLibrary.VLerp` _returnvalue_2 _returnvalue _track)))
        (:`Finished`
          (`KismetSystemLibrary.Delay` 2.0)
          (`self.FollowSpline`))))
    (:`else`)))

(event `StartMove`
  (`/Engine/EditorBlueprintResources/StandardMacros.DoOnce` false
    (:`Completed`
      (`self.FollowSpline`))))

(fn `UserConstructionScript`)