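; BP_MoveBlock is a tutorial level-design interactable that slides its Cube to the position of its Scene component.
; STARTINTERACTION passes a DoOnce gate, stores the cube's world location, then plays a timeline that lerps it toward Scene, teleporting without sweep.
; The timeline play rate is the inverse of Speed, so higher values mean slower moves.
; On finish, the gate resets only if CanBeRetriggerable is set.
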(event `/Game/Interactif/BPI_Interactible.START_INTERACTION`
  (bind _cube (`self.Cube`))
  ;[1 1 1 1 1000] ton père remy
  (`/Engine/EditorBlueprintResources/StandardMacros.DoOnce` false :!label _label
    (:`Completed`
      (`TimelineComponent.SetPlayRate` (`self.Timeline_Move`) (/ 1.0 (`self.speed`)))
      (bind _output_get (set `self.firstLoc` (`SceneComponent.K2_GetComponentLocation` _cube)))
      (bind (_direction _track) (`Timeline|Timeline_Move` :!via `PlayFromStart`)
        (:`Update`
          (`SceneComponent.K2_SetWorldLocation` _cube (`KismetMathLibrary.VLerp` _output_get (`SceneComponent.K2_GetComponentLocation` (`self.Scene`)) _track) false true))
        (:`Finished`
          (if (`self.canBeRetriggerable`)
            (goto _label :!via `Reset`)))))))

(fn `UserConstructionScript`)