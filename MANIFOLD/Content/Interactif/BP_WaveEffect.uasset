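; Shockwave effect actor that drives a tessellated plane material, with controller rumble and camera shake on activation.
; Construction builds a dynamic material from MaterialData and encodes the actor's up vector as a color for tessellation orientation.
; EnableWave animates radius and orientation through a timeline, and DisableWave fades intensity out.
; Outside 4D state it starts on BeginPlay and destroys itself after its lifetime and fade; in 4D state neither happens automatically.
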(event `self.ReceiveBeginPlay`
  (if (not (`.Is4DState_40_0D6DAE2C432995288E02B0B19198A8C4` (break `/Game/Interactif/S_ShockWave` (`self.MaterialData`))))
    (`self.EnableWave`)))

(event `EnableWave`
  (bind (_is4dstate _lifetime _emissivewidth _lines _radius _speed _color _intensity) (break `/Game/Interactif/S_ShockWave` (`self.MaterialData`)))
  (bind (_is4dstate_2 _lifetime_2) (break `/Game/Interactif/S_ShockWave` (`self.MaterialData`)))
  (`PlayerController.K2_ClientPlayForceFeedback` (`GameplayStatics.GetPlayerController` 0) "/Game/Player/BattleSystem/FFE_4DState.FFE_4DState" "None" false false false)
  (`LegacyCameraShake.StartLegacyCameraShake` (`GameplayStatics.GetPlayerCameraManager` 0) "/Game/Player/BattleSystem/LCS_4DState.LCS_4DState_C")
  (`MaterialInstanceDynamic.SetScalarParameterValue` (`self.MI_Shockwave`) "Intensity" _intensity)
  (bind (_direction _newtrack_0) (`Timeline|TL_EnableWave` :!via `PlayFromStart`)
    (:`Update`
      (`MaterialInstanceDynamic.SetScalarParameterValue` (`self.MI_Shockwave`) "Radius" (`KismetMathLibrary.Lerp` 0.0 _radius _newtrack_0))
      (`MaterialInstanceDynamic.SetVectorParameterValue` (`self.MI_Shockwave`) "TessOrientation" (`KismetMathLibrary.LinearColorLerp` (struct) (`.Color` (`self.GetTessOrientation`)) _newtrack_0))
      (if (not _is4dstate_2)
        (`KismetSystemLibrary.Delay` _lifetime_2)
        (`self.DisableWave`)))))

(event `DisableWave`
  (bind (_direction _time) (`Timeline|TL_DisableWave` :!via `PlayFromStart`)
    (:`Update`
      (`MaterialInstanceDynamic.SetScalarParameterValue` (`self.MI_Shockwave`) "Intensity" (`KismetMathLibrary.Lerp` (`.Intensity_35_356CF1144D2709F698848199E54364B5` (break `/Game/Interactif/S_ShockWave` (`self.MaterialData`))) 0.0 _time)))
    (:`Finished`
      (if (not (`.Is4DState_40_0D6DAE2C432995288E02B0B19198A8C4` (break `/Game/Interactif/S_ShockWave` (`self.MaterialData`))))
        (`self.K2_DestroyActor`)))))

(fn `GetTessOrientation`
  (returns (Vector :type "Vector Structure") (Color :type "LinearColor Structure"))
  (bind _returnvalue (`self.GetActorUpVector`))
  (bind _returnvalue_2 (`KismetMathLibrary.MakeVector` (`KismetMathLibrary.FClamp` (`KismetMathLibrary.Dot_VectorVector` _returnvalue (1.0 0.0 0.0)) -1.0) (`KismetMathLibrary.FClamp` (`KismetMathLibrary.Dot_VectorVector` _returnvalue (0.0 1.0 0.0)) -1.0) (`KismetMathLibrary.FClamp` (`KismetMathLibrary.Dot_VectorVector` _returnvalue (0.0 0.0 1.0)) -1.0)))
  (return _returnvalue_2 (`KismetMathLibrary.MakeColor` (.x _returnvalue_2) (.y _returnvalue_2) (.z _returnvalue_2))))

(fn `UserConstructionScript`
  (bind (_is4dstate _lifetime _emissivewidth _lines _radius _speed _color _intensity _height _tesswidth _basecolor _normalmap) (break `/Game/Interactif/S_ShockWave` (`self.MaterialData`)))
  (bind _returnvalue (`PrimitiveComponent.CreateDynamicMaterialInstance` (`self.Plane`) 0 "/Game/GA/Materials/VFX/MI/MI_Chockwave03.MI_Chockwave03" "None"))
  (set `self.MI_Shockwave` _returnvalue)
  (`MaterialInstanceDynamic.SetScalarParameterValue` (`self.MI_Shockwave`) "EmissiveWidth" _emissivewidth)
  (`MaterialInstanceDynamic.SetScalarParameterValue` (`self.MI_Shockwave`) "Lines" _lines)
  (`MaterialInstanceDynamic.SetScalarParameterValue` (`self.MI_Shockwave`) "Radius" _radius)
  (`MaterialInstanceDynamic.SetScalarParameterValue` (`self.MI_Shockwave`) "Speed" _speed)
  (`MaterialInstanceDynamic.SetVectorParameterValue` (`self.MI_Shockwave`) "Color" _color)
  (`MaterialInstanceDynamic.SetVectorParameterValue` (`self.MI_Shockwave`) "TessOrientation" (`.Color` (`self.GetTessOrientation`)))
  (`MaterialInstanceDynamic.SetScalarParameterValue` (`self.MI_Shockwave`) "Height" _height)
  (`MaterialInstanceDynamic.SetScalarParameterValue` (`self.MI_Shockwave`) "TessWidth" _tesswidth)
  (`MaterialInstanceDynamic.SetTextureParameterValue` (`self.MI_Shockwave`) "BaseColor" _basecolor)
  (`MaterialInstanceDynamic.SetTextureParameterValue` (`self.MI_Shockwave`) "NormalMap" _normalmap)
  (`MaterialInstanceDynamic.SetScalarParameterValue` (`self.MI_Shockwave`) "Intensity" _intensity))