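; BP_CollectItem is an interactible collectable actor that reports its interaction to the BP_CollectableParent actor that parents it.
; On BeginPlay it initializes ACInteractible with the InteractorWidget and caches the parent actor as OwnerBP.
; Starting an interaction runs once: it disables the interactible state, hides it and calls StartEventInteractMessage on the owner.
; A separate event toggles the interact icon through the same component.
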(event `/Game/Interactif/BPI_Interactible.START_INTERACTION`
  (bind _ac_interactible (`self.AC_Interactible`))
  (`/Engine/EditorBlueprintResources/StandardMacros.DoOnce` false
    (:`Completed`
      (`/Game/Interactif/AC_Interactible.ChangeState` _ac_interactible false)
      (`/Game/Interactif/AC_Interactible.Show` _ac_interactible false false)
      (message `/Game/Interactif/BPI_ActorInteract.StartEventInteract` (`self.OwnerBP`) 0))))

(event `/Game/Interactif/BPI_Interactible.ShowInteractIcon`
  (params (`On?` :type Boolean))
  ;[1 1 1] ToCopy
  (`/Game/Interactif/AC_Interactible.Show` (`self.AC_Interactible`) `On?` false))

(event `self.ReceiveBeginPlay`
  ;[1 1 1] ToCopy
  (`/Game/Interactif/AC_Interactible.Init` (`self.AC_Interactible`) (`self.InteractorWidget`))
  (bind _asbp_collectable_parent (cast `/Game/Interactif/Collectable/BP_CollectableParent` (`self.GetParentActor`)))
  (set `self.OwnerBP` _asbp_collectable_parent))

(fn `UserConstructionScript`)