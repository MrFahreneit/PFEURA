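; BP_CollectOutfit is an interactive collectable that grants the player experience when picked up.
; A weapon data table row supplies its decal material, set in the construction script and again at BeginPlay, which also stores the row's stats and hands a movement point to the interactible component.
; Collecting activates that component's movement, plays the player's collect montage, then after a short delay awards the experience and destroys the actor.
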(event `self.ReceiveBeginPlay`
  (bind (_currentweapon_datatable _currentweapon_rowname) (break `DataTableRowHandle` (`self.CurrentWeapon`)))
  (`parent.ReceiveBeginPlay`)
  (bind _returnvalue (`|GetDataTableRow` _currentweapon_datatable _currentweapon_rowname)
    (:`then`
      (set `self.WeaonStat` _returnvalue)
      (`DecalComponent.SetDecalMaterial` (`self.Decal`) (`.Decal_7_05C04F244FBE43AC007FE0BA66FC42E9` (break `/Game/Interactif/Collectable/S_WeaponStat` _returnvalue)))
      (set `/Game/Interactif/AC_Interactible.ObjectifMovement` (`self.MovementPoint`) (`self.AC_Interactible`)))))

(event `self.DoCollectAction`
  (`parent.DoCollectAction`)
  (bind _asbp_player (cast `/Game/Player/BP_Player` (`GameplayStatics.GetPlayerCharacter` 0)))
  (`/Game/Interactif/AC_Interactible.ActivateMovement` (`self.AC_Interactible`))
  (`|PlayMontage` (`Character.Mesh` _asbp_player) "/Game/GA/Skeletal/Player/A_Player_CollectItem_Montage.A_Player_CollectItem_Montage"
    (:`then`
      (`KismetSystemLibrary.Delay` 0.9)
      (`/Game/Player/BP_Player.GainExp` _asbp_player (`self.ExpToGive`))
      (`self.K2_DestroyActor`))))

(event `/Game/Interactif/BPI_ActorInteract.StartEventInteract`
  (params (value :type Integer))
  (`parent.StartEventInteract` value))

(fn `UserConstructionScript`
  (bind (_currentweapon_datatable _currentweapon_rowname) (break `DataTableRowHandle` (`self.CurrentWeapon`)))
  (`parent.UserConstructionScript`)
  (bind _returnvalue (`|GetDataTableRow` _currentweapon_datatable _currentweapon_rowname)
    (:`then`
      (`DecalComponent.SetDecalMaterial` (`self.Decal`) (`.Decal_7_05C04F244FBE43AC007FE0BA66FC42E9` (break `/Game/Interactif/Collectable/S_WeaponStat` _returnvalue))))))