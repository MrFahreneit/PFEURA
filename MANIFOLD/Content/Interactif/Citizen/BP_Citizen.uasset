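; Decal-based citizen character that shows a Peace, Fight or Win look and hops when the 2D player overlaps it outside of Fight.
; ChangeCitizenState swaps textures on a dynamic decal material, with a self-repeating tilt wobble in Peace and two alternating textures in Win.
; BeginPlay randomizes scale, roll, timings and jump height so each citizen differs.
; Jumps run on a timeline, gated by a DoOnce until finished.
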(event `self.ReceiveBeginPlay`
  (bind _returnvalue (`DecalComponent.CreateDynamicMaterialInstance` (`self.Decal`)))
  (set `self.Mat` _returnvalue)
  (`self.ChangeCitizenState` "NewEnumerator0")
  (set `self.ChangeTime` (`KismetMathLibrary.RandomFloatInRange` 0.2 1.2))
  (`SceneComponent.SetRelativeScale3D` (`self.ScalePoint`) (`KismetMathLibrary.MakeVector` 1.0 (`KismetMathLibrary.RandomFloatInRange` 0.9 1.1) (`KismetMathLibrary.RandomFloatInRange` 0.9 1.1)))
  (`SceneComponent.K2_SetRelativeRotation` (`self.ScalePoint`) (`KismetMathLibrary.MakeRotator` (`KismetMathLibrary.RandomFloatInRange` -3.0 3.0)) false false)
  (set `self.RandomIdle` (* (`self.RandomIdle`) (`KismetMathLibrary.RandomFloatInRange` 0.7 1.3)))
  (set `self.JumpHeight` (* (`self.JumpHeight`) (`KismetMathLibrary.RandomFloatInRange` 0.7 1.3))))

(event `MoveIdle`
  (bind _scalepoint (`self.ScalePoint`))
  (`/Engine/EditorBlueprintResources/StandardMacros.FlipFlop`
    (:`A`
      (`SceneComponent.K2_SetRelativeRotation` _scalepoint (struct :`Pitch` 5.0) false false))
    (:`B`
      (`SceneComponent.K2_SetRelativeRotation` _scalepoint (struct :`Pitch` -5.0) false false)))
  (if (`|EnumEquality` (`self.CurrentState`) "NewEnumerator0")
    (`KismetSystemLibrary.Delay` (`self.RandomIdle`))
    (`self.MoveIdle`)))

(event `ChangeCitizenState`
  (params (CurrentState :type "/Game/Interactif/Citizen/Enum_CitizenState Enum" :default "NewEnumerator0"))
  (bind _output_get (set `self.CurrentState` CurrentState))
  (switch `/Game/Interactif/Citizen/Enum_CitizenState` _output_get
    (:`NewEnumerator0`
      (`MaterialInstanceDynamic.SetTextureParameterValue` (`self.Mat`) "BaseColor" (`self.PeaceText`))
      (`MaterialInstanceDynamic.SetTextureParameterValue` (`self.Mat`) "OpacityMap" (`self.PeaceText`))
      (`self.MoveIdle`))
    (:`NewEnumerator1`
      (`MaterialInstanceDynamic.SetTextureParameterValue` (`self.Mat`) "BaseColor" (`self.FightTxt`))
      (`MaterialInstanceDynamic.SetTextureParameterValue` (`self.Mat`) "OpacityMap" (`self.FightTxt`))
      (`SceneComponent.K2_SetRelativeRotation` (`self.ScalePoint`) (struct) false false))
    (:`NewEnumerator2`
      (`self.ChangeWinSprite`))))

(event `ChangeWinSprite`
  (bind _isa (`/Engine/EditorBlueprintResources/StandardMacros.FlipFlop`)
    (:`A`
      _)
    (:`B`
      _))
  (`MaterialInstanceDynamic.SetTextureParameterValue` (`self.Mat`) "BaseColor" (select `bool` _isa :`false` (`self.WinTxt1`) :`true` (`self.WinTxt2`)))
  (`MaterialInstanceDynamic.SetTextureParameterValue` (`self.Mat`) "OpacityMap" (select `bool` _isa :`false` (`self.WinTxt1`) :`true` (`self.WinTxt2`)))
  (`KismetSystemLibrary.Delay` (`self.ChangeTime`))
  (`self.ChangeWinSprite`))

(event `self.Box.OnComponentBeginOverlap`
  (params (OverlappedComponent :type "PrimitiveComponent Object Reference") (OtherActor :type "Actor Object Reference") (OtherComp :type "PrimitiveComponent Object Reference") (OtherBodyIndex :type Integer) (bFromSweep :type Boolean) (SweepResult :type "HitResult Structure (by ref)"))
  (bind _currentstate (`self.CurrentState`))
  (cast `/Game/Player/2DPlayer/BP_2DPlayer` OtherActor)
  (if (or (`|EnumEquality` _currentstate "NewEnumerator0") (`|EnumEquality` _currentstate "NewEnumerator2"))
    (`self.Jump`)))

(event `Jump`
  (`/Engine/EditorBlueprintResources/StandardMacros.DoOnce` false :!label _label
    (:`Completed`
      (`TimelineComponent.SetPlayRate` (`self.JumpTimeline`) (/ 1.0 0.5))
      (bind _output_get (set `self.PointA` (`SceneComponent.RelativeLocation` (`self.JumpPoint`))))
      (set `self.PointB` (+ _output_get (`KismetMathLibrary.MakeVector` (`self.JumpHeight`))))
      (bind (_direction _alpha) (`Timeline|JumpTimeline` :!via `PlayFromStart`)
        (:`Update`
          (`SceneComponent.K2_SetRelativeLocation` (`self.JumpPoint`) (`KismetMathLibrary.VLerp` (`self.PointA`) (`self.PointB`) _alpha) false false))
        (:`Finished`
          (goto _label :!via `Reset`))))))

(fn `UserConstructionScript`)